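; BP_SkyLightCapture is an editor tool that poses a procedural sky at set times of day for cubemap capture.
; Its construction script restricts the cube capture component to the Sky actor and maps the chosen cubemap index to evenly spaced times from 0 to 12.
; Entering capture mode saves the sky's time of day.
; Leaving it restores that time, recaptures the sky and updates the skylight.
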(fn `UserConstructionScript`
  (bind _sky (`self.Sky`))
  (bind _capturecubemapcount (`self.CaptureCubemapCount`))
  (bind _returnvalue (* (- (`self.CaptureCubemapIndex`) 1) (/ 12.0 (`KismetMathLibrary.Conv_IntToDouble` (- _capturecubemapcount 1)))))
  (set `self.Generate` false)
  (set `SceneCaptureComponent.ShowOnlyActors` (`|MakeArray` (`self.Sky`) :!type "Actor Object Reference") (`self.CaptureComponentCube`))
  (set `self.CaptureCubemapIndex` (`KismetMathLibrary.Min` (`self.CaptureCubemapIndex`) (`self.CaptureCubemapCount`)))
  (`/Engine/EditorBlueprintResources/StandardMacros.IsValid` (`self.Sky`)
    (:`Is Valid`
      (if (!= (`self.CaptureMode`) (`self.CaptureModeActive`))
        (set `self.CaptureModeActive` (`self.CaptureMode`))
        (if (`self.CaptureMode`)
          ;[1 1 1] Save for capture
          (set `self.CaptureSavedTimeOfDay` (`/Game/FastStylizedProceduralSky2/BP_FastStylizedProceduralSky.TimeOfDay` (`self.Sky`)))
          (switch `int` _capturecubemapcount :!label _label
            (:`Default`
              (`/Game/FastStylizedProceduralSky2/BP_FastStylizedProceduralSky.SetTimeOfDay` (`self.Sky`) _returnvalue)
              (set `self.CaptureTimeDebug` _returnvalue)))
          (else
            ;[1 1 1] Load after capture
            (`/Game/FastStylizedProceduralSky2/BP_FastStylizedProceduralSky.SetTimeOfDay` _sky (`self.CaptureSavedTimeOfDay`))
            (`/Game/FastStylizedProceduralSky2/BP_FastStylizedProceduralSky.PostConstructionScript` _sky)
            (`/Game/FastStylizedProceduralSky2/BP_FastStylizedProceduralSky.RecaptureSky` _sky)
            (`/Game/FastStylizedProceduralSky2/BP_FastStylizedProceduralSky.UpdateSkyLight` _sky)))
        (elif (`self.CaptureMode`)
          (goto _label))))))