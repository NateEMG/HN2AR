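; Editor tool actor that bakes a stylized moon texture with atmosphere, detail and color controls into a render target.
; On construction and BeginPlay it pushes its settings to a dynamic material instance from its plane.
; It draws that material in two passes, a mask pass with the detail map, then a pass with the color map.
; SaveTexture saves the render target as a static Texture2D asset and prints its path.
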(event `Render`
  (`/Engine/EditorBlueprintResources/StandardMacros.IsValid` (`self.RenderTarget`)
    (:`Is Valid`
      (`MaterialInstanceDynamic.SetScalarParameterValue` (`self.MaterialInst`) "AtmosphereSize" (`self.AtmosphereSize`))
      (`MaterialInstanceDynamic.SetScalarParameterValue` (`self.MaterialInst`) "AtmosphereInShadow" (`self.AtmosphereInShadow`))
      (`MaterialInstanceDynamic.SetScalarParameterValue` (`self.MaterialInst`) "DetailScale" (`self.DetailScale`))
      (`MaterialInstanceDynamic.SetScalarParameterValue` (`self.MaterialInst`) "TetureResolution" (* (`self.TextureSize`) (`self.SampleResolution`)))
      (`MaterialInstanceDynamic.SetScalarParameterValue` (`self.MaterialInst`) "ColorBase" (`self.ColorBase`))
      (`MaterialInstanceDynamic.SetScalarParameterValue` (`self.MaterialInst`) "ColorScale" (`self.ColorScale`))
      (`MaterialInstanceDynamic.SetScalarParameterValue` (`self.MaterialInst`) "AtmosphereExp" (`self.AtmosphereExp`))
      (`MaterialInstanceDynamic.SetScalarParameterValue` (`self.MaterialInst`) "AtmosphereBase" (`self.AtmosphereBase`))
      (`MaterialInstanceDynamic.SetScalarParameterValue` (`self.MaterialInst`) "EdgeHardness" (`self.EdgeHardness`))
      (`MaterialInstanceDynamic.SetTextureParameterValue` (`self.MaterialInst`) "DetailMap" (`self.DetailMap`))
      (`KismetRenderingLibrary.ClearRenderTarget2D` "/Game/FastStylizedProceduralSky2/Tools/MoonCreator/RT_Moon.RT_Moon")
      (`MaterialInstanceDynamic.SetScalarParameterValue` (`self.MaterialInst`) "Mask" 1.0)
      (`self.Draw`))))

(event `self.ReceiveBeginPlay`
  (`self.Render`))

(fn `Draw`
  (`KismetRenderingLibrary.DrawMaterialToRenderTarget` (`self.RenderTarget`) (`self.MaterialInst`))
  (`MaterialInstanceDynamic.SetScalarParameterValue` (`self.MaterialInst`) "Mask" 0.0)
  (`MaterialInstanceDynamic.SetTextureParameterValue` (`self.MaterialInst`) "DetailMap" (`self.ColorMap`))
  (`KismetRenderingLibrary.DrawMaterialToRenderTarget` (`self.RenderTarget`) (`self.MaterialInst`)))

(fn `SaveTexture`
  (bind _returnvalue (`KismetRenderingLibrary.RenderTargetCreateStaticTexture2DEditorOnly` (`self.RenderTarget`) (`self.TextureName`) "TC_VectorDisplacementmap" (`self.TextureSettings`)))
  (`KismetSystemLibrary.PrintString` (`KismetSystemLibrary.GetPathName` _returnvalue)))

(fn `UserConstructionScript`
  (bind _rendertarget (`self.RenderTarget`))
  (`/Engine/EditorBlueprintResources/StandardMacros.IsValid` _rendertarget
    (:`Is Valid`
      (set `self.TextureSize` (`TextureRenderTarget2D.SizeX` _rendertarget))
      (bind _returnvalue (`PrimitiveComponent.CreateDynamicMaterialInstance` (`self.Plane`) 0 null))
      (set `self.MaterialInst` _returnvalue)
      (`self.Render`))))