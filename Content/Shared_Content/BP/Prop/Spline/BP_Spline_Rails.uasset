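; Spline rail prop that moves a referenced Actor along Spline1, oriented to the spline's tangent.
; The construction script snaps that Actor to the first spline point.
; A Timeline alpha maps to distance along the spline, with play rate set from TimelineLength, and restarts from the beginning whenever it finishes.
; PlayTimeline, Play, Stop and Reverse events control the motion; BeginPlay does not start it.
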(event `self.ReceiveBeginPlay`)

(event `Stop`
  (bind _spline1 (`self.Spline1`))
  (bind _spline1_2 (`self.Spline1`))
  (bind (_direction _alpha) (`Timeline|Timeline` :!via `Stop` :!label _label)
    (:`Update`
      (bind _returnvalue (`KismetMathLibrary.Lerp` 0.0 (`SplineComponent.GetDistanceAlongSplineAtSplinePoint` _spline1 (- (`SplineComponent.GetNumberOfSplinePoints` _spline1) 1)) _alpha))
      (`self.K2_SetActorLocation` (`self.Actor`) (`SplineComponent.GetLocationAtDistanceAlongSpline` _spline1_2 _returnvalue "World") false false)
      (`self.K2_SetActorRotation` (`self.Actor`) (`KismetMathLibrary.Conv_VectorToRotator` (`SplineComponent.GetTangentAtDistanceAlongSpline` _spline1_2 _returnvalue "World")) false))
    (:`Finished`
      (`self.Play Timeline`))))

(event `Reverse`
  (goto _label :!via `Reverse`))

(event `Play`
  (goto _label))

(event `Play Timeline`
  (`/Engine/EditorBlueprintResources/StandardMacros.IsValid` (`self.Actor`)
    (:`Is Valid`
      (`TimelineComponent.SetPlayRate` (`self.Timeline`) (/ 1.0 (`self.Timeline Length`)))
      (goto _label :!via `PlayFromStart`))))

(fn `UserConstructionScript`
  (bind _actor (`self.Actor`))
  (`parent.UserConstructionScript`)
  (`self.K2_SetActorLocation` _actor (`SplineComponent.GetLocationAtSplinePoint` (`self.Spline1`) 0 "World") false false)
  (`self.K2_SetActorRotation` _actor (`KismetMathLibrary.Conv_VectorToRotator` (`SplineComponent.GetTangentAtSplinePoint` (`self.Spline1`) 0 "World")) false))