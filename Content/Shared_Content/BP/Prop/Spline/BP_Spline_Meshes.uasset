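; Spline prop actor that builds a chain of deformed meshes along Spline1 in its construction script, with optional start and end cap meshes.
; Each segment picks a SplineMeshes entry through the per-segment MeshIndex array, which sets mesh, materials, axis, offsets and boundaries.
; Spline point roll and Y scale, multiplied by OverallThickness, shape each segment.
; Helper functions pick component templates by collision flag and Mobility.
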(fn `Add spline component`
  (params (Collision :type Boolean :default true))
  (returns (Mesh :type "SplineMeshComponent Object Reference"))
  (bind _mobility (`self.Mobility`))
  (if Collision
    (switch `EComponentMobility` _mobility
      (:`Static`
        (bind _returnvalue (`AddComponent|NODE_AddSplineMeshComponent-1`))
        (return _returnvalue))
      (:`Stationary`
        (bind _returnvalue_2 (`AddComponent|NODE_AddSplineMeshComponent-2`))
        (return _returnvalue_2))
      (:`Movable`
        (bind _returnvalue_3 (`AddComponent|NODE_AddSplineMeshComponent-3`))
        (return _returnvalue_3)))
    (else
      (switch `EComponentMobility` _mobility
        (:`Static`
          (bind _returnvalue_4 (`AddComponent|NODE_AddSplineMeshComponent-4`))
          (return _returnvalue_4))
        (:`Stationary`
          (bind _returnvalue_5 (`AddComponent|NODE_AddSplineMeshComponent-5`))
          (return _returnvalue_5))
        (:`Movable`
          (bind _returnvalue_6 (`AddComponent|NODE_AddSplineMeshComponent-6`))
          (return _returnvalue_6))))))

(fn `Add static component`
  (params (`Static mesh` :type "/Game/Shared_Content/BP/Prop/Spline/ST/Mesh Structure"))
  (returns (`Return Mesh` :type "StaticMeshComponent Object Reference"))
  (locals (Mesh :type "StaticMeshComponent Object Reference"))
  (bind (_mesh _materialsoverride _collision) (break `/Game/Shared_Content/BP/Prop/Spline/ST/Mesh` `Static mesh`))
  (bind _mobility (`self.Mobility`))
  (bind _mesh_2 (`local.Mesh`))
  (bind _mesh_3 (`local.Mesh`))
  (`|ExecutionSequence`
    (:`then_0`
      (if _collision
        (switch `EComponentMobility` _mobility
          (:`Static`
            (bind _returnvalue (`AddComponent|NODE_AddStaticMeshComponent-0`))
            (set `local.Mesh` _returnvalue))
          (:`Stationary`
            (bind _returnvalue_2 (`AddComponent|NODE_AddStaticMeshComponent-1`))
            (set `local.Mesh` _returnvalue_2))
          (:`Movable`
            (bind _returnvalue_3 (`AddComponent|NODE_AddStaticMeshComponent-2`))
            (set `local.Mesh` _returnvalue_3)))
        (else
          (switch `EComponentMobility` _mobility
            (:`Static`
              (bind _returnvalue_4 (`AddComponent|NODE_AddStaticMeshComponent-3`))
              (set `local.Mesh` _returnvalue_4))
            (:`Stationary`
              (bind _returnvalue_5 (`AddComponent|NODE_AddStaticMeshComponent-4`))
              (set `local.Mesh` _returnvalue_5))
            (:`Movable`
              (bind _returnvalue_6 (`AddComponent|NODE_AddStaticMeshComponent-5`))
              (set `local.Mesh` _returnvalue_6))))))
    (:`then_1`
      (`StaticMeshComponent.SetStaticMesh` _mesh_2 _mesh)
      (for (_array_element _array_index) _materialsoverride
        (if (not (> _array_index (`PrimitiveComponent.GetNumMaterials` _mesh_2)))
          (`PrimitiveComponent.SetMaterial` _mesh_2 _array_index _array_element)
          (else
            (break))))
      (`PrimitiveComponent.SetWalkableSlopeOverride` _mesh_3 (`self.Walkable Slope Override`))
      (return _mesh_3))))

(fn `UserConstructionScript`
  (bind _spline1 (`self.Spline1`))
  (bind _mesh_index (`self.Mesh index`))
  (bind _spline_meshes (`self.Spline Meshes`))
  (bind _end_mesh_static (`self.End mesh static`))
  (bind _start_mesh_static (`self.Start mesh static`))
  (bind _returnvalue (`SplineComponent.GetNumberOfSplinePoints` (`self.Spline1`)))
  (bind _returnvalue_2 (- _returnvalue 2))
  (bind _returnvalue_3 (- _returnvalue 1))
  (bind _returnvalue_4 (* (.y (.scale (`SplineComponent.GetTransformAtSplinePoint` (`self.Spline1`) 0 "World" true))) (`self.Overall Thickness`)))
  (bind _returnvalue_5 (* (.y (.scale (`SplineComponent.GetTransformAtSplinePoint` (`self.Spline1`) _returnvalue_3 "World" true))) (`self.Overall Thickness`)))
  (`|ExecutionSequence`
    (:`then_0`
      (for _array_element (`self.Meshes`)
        (`ActorComponent.K2_DestroyComponent` _array_element))
      (`KismetArrayLibrary.Array_Clear` (`self.Meshes`)))
    (:`then_1`
      (`KismetArrayLibrary.Array_Resize` _mesh_index _returnvalue_3)
      (for _index (range (+ _returnvalue_2 1))
        (bind _output (`|GetArrayItem` _mesh_index _index))
        (bind (_mesh _materialsoverride _forwardaxis _updirection _splineboundarymin _splineboundarymax _startoffset _endoffset _collision) (break `/Game/Shared_Content/BP/Prop/Spline/ST/SplineMesh` (`|GetArrayItem` _spline_meshes _output)))
        (if (and (not (> _output (`KismetArrayLibrary.Array_LastIndex` _spline_meshes))) (`KismetSystemLibrary.IsValid` _mesh))
          (bind _returnvalue_6 (and _collision (`self.Update Meshes (see tooltip)`)))
          (bind _mesh_2 (`self.Add spline component` _returnvalue_6))
          (`KismetArrayLibrary.Array_Add` (`self.Meshes`) _mesh_2)
          (`StaticMeshComponent.SetStaticMesh` _mesh_2 _mesh)
          (`PrimitiveComponent.SetWalkableSlopeOverride` _mesh_2 (`self.Walkable Slope Override`))
          (for (_array_element_2 _array_index) _materialsoverride
            (if (not (> _array_index (`PrimitiveComponent.GetNumMaterials` _mesh_2)))
              (`PrimitiveComponent.SetMaterial` _mesh_2 _array_index _array_element_2)
              (else
                (break))))
          (`SplineMeshComponent.SetForwardAxis` _mesh_2 _forwardaxis _returnvalue_6)
          (`SplineMeshComponent.SetStartRoll` _mesh_2 (/ (.roll (`SplineComponent.GetRotationAtSplinePoint` _spline1 _index "Local")) 55.0) _returnvalue_6)
          (bind _returnvalue_7 (+ _index 1))
          (`SplineMeshComponent.SetEndRoll` _mesh_2 (/ (.roll (`SplineComponent.GetRotationAtSplinePoint` _spline1 _returnvalue_7 "Local")) 55.0) _returnvalue_6)
          (bind _returnvalue_8 (* (.y (`SplineComponent.GetScaleAtSplinePoint` _spline1 _index)) (`self.Overall Thickness`)))
          (`SplineMeshComponent.SetStartScale` _mesh_2 (`KismetMathLibrary.MakeVector2D` _returnvalue_8 _returnvalue_8) _returnvalue_6)
          (bind _returnvalue_9 (* (.y (`SplineComponent.GetScaleAtSplinePoint` _spline1 _returnvalue_7)) (`self.Overall Thickness`)))
          (`SplineMeshComponent.SetEndScale` _mesh_2 (`KismetMathLibrary.MakeVector2D` _returnvalue_9 _returnvalue_9) _returnvalue_6)
          (`SplineMeshComponent.SetSplineUpDir` _mesh_2 _updirection _returnvalue_6)
          (`SplineMeshComponent.SetBoundaryMin` _mesh_2 _splineboundarymin _returnvalue_6)
          (`SplineMeshComponent.SetBoundaryMax` _mesh_2 _splineboundarymax _returnvalue_6)
          (`SplineMeshComponent.SetStartOffset` _mesh_2 _startoffset _returnvalue_6)
          (`SplineMeshComponent.SetEndOffset` _mesh_2 _endoffset _returnvalue_6)
          (bind (_location _tangent) (`SplineComponent.GetLocationAndTangentAtSplinePoint` _spline1 _index "Local"))
          (bind (_location_2 _tangent_2) (`SplineComponent.GetLocationAndTangentAtSplinePoint` _spline1 _returnvalue_7 "Local"))
          (`SplineMeshComponent.SetStartAndEnd` _mesh_2 _location _tangent _location_2 _tangent_2 _returnvalue_6))
        (if (and (`KismetSystemLibrary.IsValid` (`.Mesh_2_AF6621E7488F18D7AA9F36920574E737` (break `/Game/Shared_Content/BP/Prop/Spline/ST/Mesh` _start_mesh_static))) (== _index 0))
          (bind _return_mesh (`self.Add static component` _start_mesh_static))
          (`KismetArrayLibrary.Array_Add` (`self.Meshes`) _return_mesh)
          (`SceneComponent.K2_SetWorldTransform` _return_mesh (`KismetMathLibrary.MakeTransform` (.location (`SplineComponent.GetTransformAtSplinePoint` (`self.Spline1`) 0 "World" true)) (.rotation (`SplineComponent.GetTransformAtSplinePoint` (`self.Spline1`) 0 "World" true)) (`KismetMathLibrary.MakeVector` _returnvalue_4 _returnvalue_4 (.z (.scale (`SplineComponent.GetTransformAtSplinePoint` (`self.Spline1`) 0 "World" true))))) false false))
        (if (and (`KismetSystemLibrary.IsValid` (`.Mesh_2_AF6621E7488F18D7AA9F36920574E737` (break `/Game/Shared_Content/BP/Prop/Spline/ST/Mesh` _end_mesh_static))) (== _index _returnvalue_2))
          (bind _return_mesh_2 (`self.Add static component` _end_mesh_static))
          (`KismetArrayLibrary.Array_Add` (`self.Meshes`) _return_mesh_2)
          (`SceneComponent.K2_SetWorldTransform` _return_mesh_2 (`KismetMathLibrary.MakeTransform` (.location (`SplineComponent.GetTransformAtSplinePoint` (`self.Spline1`) _returnvalue_3 "World" true)) (.rotation (`SplineComponent.GetTransformAtSplinePoint` (`self.Spline1`) _returnvalue_3 "World" true)) (`KismetMathLibrary.MakeVector` _returnvalue_5 _returnvalue_5 (.z (.scale (`SplineComponent.GetTransformAtSplinePoint` (`self.Spline1`) _returnvalue_3 "World" true))))) false false))))))