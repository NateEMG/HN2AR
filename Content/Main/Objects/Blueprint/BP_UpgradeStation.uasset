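; BP_UpgradeStation is a world station where the player upgrades their Sedan van using deposited scrap.
; One trigger box tracks whether a Sedan is parked inside and keeps a reference to it.
; A second box consumes overlapping BP_Scrap after a short delay, increments the scrap count and briefly flashes a text render.
; Interacting with the table while a car is present opens BPW_UpgradeVan with the van, scrap and station, switching to UI-only input.
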(event `self.ReceiveBeginPlay`)

(event `/Game/Main/Characters/Quentin/Blueprint/Interaction_Interface.Interact`
  (params (Component :type "ActorComponent Object Reference"))
  (bind _returnvalue (`GameplayStatics.GetPlayerController` 0))
  (if (== Component (`self.Table`))
    (if (`self.CarInStation?`)
      (bind _returnvalue_2 (`|CreateWidget` "/Game/UI/Widget/BPW_UpgradeVan.BPW_UpgradeVan_C" (`GameplayStatics.GetPlayerController` 0)))
      (set `/Game/UI/Widget/BPW_UpgradeVan.VanRef` (stale `self.Box.OnComponentBeginOverlap` _output_get) _returnvalue_2)
      (set `/Game/UI/Widget/BPW_UpgradeVan.ScrapAmount` (`self.ScrapAmount`) _returnvalue_2)
      (set `/Game/UI/Widget/BPW_UpgradeVan.UpgradeStation` self _returnvalue_2)
      (`UserWidget.AddToViewport` _returnvalue_2 0)
      (`WidgetBlueprintLibrary.SetInputMode_UIOnlyEx` _returnvalue _returnvalue_2)
      (set `PlayerController.bShowMouseCursor` true _returnvalue))))

(event `self.Box.OnComponentBeginOverlap`
  (params (OverlappedComponent :type "PrimitiveComponent Object Reference") (OtherActor :type "Actor Object Reference") (OtherComp :type "PrimitiveComponent Object Reference") (OtherBodyIndex :type Integer) (bFromSweep :type Boolean) (SweepResult :type "HitResult Structure (by ref)"))
  (bind _assedan (cast `/Game/VehicleBP/Sedan/Sedan` OtherActor))
  (set `self.CarInStation?` true)
  (bind _output_get (set `self.VanRef` _assedan)))

(event `self.Box.OnComponentEndOverlap`
  (params (OverlappedComponent :type "PrimitiveComponent Object Reference") (OtherActor :type "Actor Object Reference") (OtherComp :type "PrimitiveComponent Object Reference") (OtherBodyIndex :type Integer))
  (cast `/Game/VehicleBP/Sedan/Sedan` OtherActor)
  (set `self.CarInStation?` false)
  (set `self.VanRef` null))

(event `self.Box1.OnComponentBeginOverlap`
  (params (OverlappedComponent :type "PrimitiveComponent Object Reference") (OtherActor :type "Actor Object Reference") (OtherComp :type "PrimitiveComponent Object Reference") (OtherBodyIndex :type Integer) (bFromSweep :type Boolean) (SweepResult :type "HitResult Structure (by ref)"))
  (bind _textrender1 (`self.TextRender1`))
  (bind _asbp_scrap (cast `/Game/Main/Objects/Blueprint/BP_Scrap` OtherActor))
  (set `/Game/Main/Objects/Blueprint/BP_Base_Item.Can Pick Up` false _asbp_scrap)
  (`KismetSystemLibrary.Delay` 0.5)
  (`self.K2_DestroyActor` _asbp_scrap)
  (`/Engine/EditorBlueprintResources/StandardMacros.IncrementInt` (`self.ScrapAmount`)
    (:`  `
      (`SceneComponent.SetVisibility` _textrender1 true false)
      (`KismetSystemLibrary.Delay` 1.0)
      (`SceneComponent.SetVisibility` _textrender1 false false))))

(fn `UserConstructionScript`)