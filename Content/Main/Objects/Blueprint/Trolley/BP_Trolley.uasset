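; Trolley actor with forward and reverse levers that start and stop its movement through a Rails reference.
; Interact maps the used lever to MoveLever, which toggles On and either stops Rails and resets both levers, or tilts that lever and sets TrolleyMovement.
; The first start calls PlayTimeline on Rails, while later starts call Play or Reverse by direction.
; MoveComponentTo eases the lever rotations.
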(event `Move Lever`
  (params (Forward :type Boolean))
  (bind _rails (`self.Rails`))
  (bind _first_time (`self.First Time`))
  (if (`self.On`)
    (set `self.On` false)
    (`self.Reset Lever Rotation`)
    (`/Game/Shared_Content/BP/Prop/Spline/BP_Spline_Rails.Stop` (`self.Rails`))
    (else
      (set `self.On` true)
      (if Forward
        (`self.Rotate Lever` (`self.Lever_F`))
        (if _first_time
          (set `self.First Time` false)
          (set `self.Trolley Movement` "NewEnumerator0")
          (`/Game/Shared_Content/BP/Prop/Spline/BP_Spline_Rails.Play Timeline` (`self.Rails`))
          (else
            (set `self.Trolley Movement` "NewEnumerator0")
            (`/Game/Shared_Content/BP/Prop/Spline/BP_Spline_Rails.Play` _rails)))
        (else
          (`self.Rotate Lever` (`self.Lever_R`))
          (if _first_time
            (set `self.First Time` false)
            (set `self.Trolley Movement` "NewEnumerator1")
            (`/Game/Shared_Content/BP/Prop/Spline/BP_Spline_Rails.Play Timeline` (`self.Rails`))
            (else
              (set `self.Trolley Movement` "NewEnumerator1")
              (`/Game/Shared_Content/BP/Prop/Spline/BP_Spline_Rails.Reverse` _rails))))))))

(event `Rotate Lever`
  (params (Lever :type "SceneComponent Object Reference") (Forward :type Boolean))
  (bind _relativelocation (`SceneComponent.RelativeLocation` Lever))
  (`/Engine/EditorBlueprintResources/StandardMacros.DoOnce` false :!label _label
    (:`Completed`
      (if Forward
        (`KismetSystemLibrary.MoveComponentTo` Lever _relativelocation (struct :`Pitch` 20.0) false true 0.2 true)
        (goto _label :!via `Reset`)
        (else
          (`KismetSystemLibrary.MoveComponentTo` Lever _relativelocation (struct :`Pitch` -20.0) false true 0.2 true)
          (goto _label :!via `Reset`))))))

(event `/Game/Main/Characters/Quentin/Blueprint/Interaction_Interface.Interact`
  (params (Component :type "ActorComponent Object Reference"))
  (if (== Component (`self.Lever_F`))
    (`self.Move Lever` true)
    (elif (== Component (`self.Lever_R`))
      (`self.Move Lever` false))))

(event `Reset Lever Rotation`
  (bind _lever_r (`self.Lever_R`))
  (bind _lever_f (`self.Lever_F`))
  (`|ExecutionSequence`
    (:`then_0`
      (`KismetSystemLibrary.MoveComponentTo` _lever_f (`SceneComponent.RelativeLocation` _lever_f) (struct) false true 0.2 true))
    (:`then_1`
      (`KismetSystemLibrary.MoveComponentTo` _lever_r (`SceneComponent.RelativeLocation` _lever_r) (struct) false true 0.2 true))))

(fn `UserConstructionScript`)