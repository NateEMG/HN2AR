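; BP_Binoculars is a binoculars item for the Quentin character that toggles an animation task when used.
; On socket creation it sets its Socket from Quentin's Items.
; Use flips Quentin's AnimTask between two enum states, leaving any visible effect to logic outside this Blueprint.
; The interaction event has no effect, and the default events are disabled.
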(event `self.Run Socket Creation`
  (set `self.Socket` (`/Game/Main/Characters/Quentin/Blueprint/CH_Quentin.Items` (`self.Quentin`))))

(event `self.Run Interaction`
  (if true
    _))

(event `self.Use`
  (bind _quentin (`self.Quentin`))
  (if (`|EnumEquality` (`/Game/Main/Characters/Quentin/Blueprint/CH_Quentin.Anim Task` (`self.Quentin`)) "NewEnumerator5")
    (set `/Game/Main/Characters/Quentin/Blueprint/CH_Quentin.Anim Task` "NewEnumerator1" _quentin)
    (else
      (set `/Game/Main/Characters/Quentin/Blueprint/CH_Quentin.Anim Task` "NewEnumerator5" _quentin))))

(fn `UserConstructionScript`
  (`parent.UserConstructionScript`))