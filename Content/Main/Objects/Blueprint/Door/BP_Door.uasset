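; Interactive hinged door that the player and BP_Base_AI characters open inward or outward, with movement-driven swing and sounds.
; On BeginPlay it spawns a BP_SmartLinkDoor, then a looping timer syncs that link and AI access with Locked.
; Player interaction toggles the door, picking swing direction from a Box overlap.
; Two AI trigger boxes share gates, align the AI, play an opening montage, then auto-close the door.
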(event `self.ReceiveBeginPlay`
  (bind (_returnvalue_roll _returnvalue_pitch _returnvalue_yaw) (`KismetMathLibrary.BreakRotator` (`self.K2_GetActorRotation`)))
  (`parent.ReceiveBeginPlay`)
  (bind _returnvalue (`|SpawnActorFromClass` "/Game/Main/Objects/Blueprint/Door/BP_SmartLinkDoor.BP_SmartLinkDoor_C" (`KismetMathLibrary.MakeTransform` (`self.K2_GetActorLocation`) (`KismetMathLibrary.MakeRotator` _returnvalue_roll _returnvalue_pitch (+ _returnvalue_yaw 90.0))) "AlwaysSpawn" "OverrideRootScale" null null))
  (bind _output_get (set `self.Link` _returnvalue))
  (`NavLinkProxy.SetSmartLinkEnabled` _output_get true)
  (`KismetSystemLibrary.Delay` 2.0)
  (`self.Tick`))

(event `Tick`
  (bind _link (`self.Link`))
  (`KismetSystemLibrary.K2_SetTimerDelegate` (delegate `Tick`) 0.5 true 0.5 0.5)
  (if (`self.Locked`)
    (`/Engine/EditorBlueprintResources/StandardMacros.DoOnce` false :!label _label
      (:`Completed`
        (set `self.AI Can Open?` false)
        (`NavLinkProxy.SetSmartLinkEnabled` _link false)
        (goto _label_2 :!via `Reset`)))
    (else
      (`/Engine/EditorBlueprintResources/StandardMacros.DoOnce` false :!label _label_2
        (:`Completed`
          (set `self.AI Can Open?` true)
          (`NavLinkProxy.SetSmartLinkEnabled` _link true)
          (goto _label :!via `Reset`))))))

(event `Close Door`
  (bind _door (`self.Door`))
  (bind _door_2 (`self.Door`))
  (bind _door_3 (`self.Door`))
  (`|ExecutionSequence`
    (:`then_0`
      (goto _label_4 :!via `Stop`))
    (:`then_1`
      (goto _label_5 :!via `Stop`))
    (:`then_2`
      (set `self.Open` false)
      (`AudioComponent.Play` (`self.Closing Audio`) 0.0)
      (`KismetSystemLibrary.MoveComponentTo` _door_3 (`SceneComponent.RelativeLocation` _door_3) (struct) false false (`self.Over Time`) true :!label _label_3)
      (`AudioComponent.FadeOut` (`self.Closing Audio`) 0.2 0.0 "Linear")
      (if (`self.Open`)
        (set `self.Close Full` false)
        (else
          (set `self.Close Full` true)
          (`GameplayStatics.PlaySoundAtLocation` (`self.Closed`) (`SceneComponent.K2_GetComponentLocation` (`self.Door`)) (struct) 1.0 1.0 0.0 null null null))))))

(event `/Game/Main/Characters/Quentin/Blueprint/Interaction_Interface.Interact`
  (params (Component :type "ActorComponent Object Reference"))
  (if (== Component (`self.Door`))
    (`self.Open Door` (`self.Quentin`))))

(event `Open Door`
  (params (Actor :type "Actor Object Reference"))
  (if (`self.Locked`)
    (`GameplayStatics.PlaySoundAtLocation` (`self.Lock`) (`SceneComponent.K2_GetComponentLocation` (`self.Door`)) (struct) 1.0 1.0 0.0 null null null)
    (elif (`self.Open`)
      (`self.Close Door`)
      (else
        (`|ExecutionSequence`
          (:`then_0`
            (goto _label_3 :!via `Stop`))
          (:`then_1`
            (set `self.Open` true)
            (if (`PrimitiveComponent.IsOverlappingActor` (`self.Box`) Actor)
              (`self.Open Door Outward`)
              (else
                (`self.Open Door Inward`)))))))))

(event `Stop`
  (bind _door (`self.Door`))
  (bind _door_2 (`self.Door`))
  (`|ExecutionSequence`
    (:`then_0`
      (goto _label_3 :!via `Stop`))
    (:`then_1`
      (goto _label_4 :!via `Stop`))
    (:`then_2`
      (goto _label_5 :!via `Stop`))))

(event `Open Door Inward`
  (bind _door (`self.Door`))
  (`self.Play Sound Effect`)
  (`self.Stop`)
  (`KismetSystemLibrary.MoveComponentTo` _door (`SceneComponent.RelativeLocation` _door) (struct :`Yaw` 100.0) false false (`self.Over Time`) true :!label _label_4))

(event `Open Door Outward`
  (bind _door (`self.Door`))
  (`self.Play Sound Effect`)
  (`self.Stop`)
  (`KismetSystemLibrary.MoveComponentTo` _door (`SceneComponent.RelativeLocation` _door) (struct :`Yaw` -100.0) false false (`self.Over Time`) true :!label _label_5))

(event `Play Sound Effect`
  (bind _returnvalue (`SceneComponent.K2_GetComponentLocation` (`self.Door`)))
  (if (`self.Close Full`)
    (`GameplayStatics.PlaySoundAtLocation` (`self.Opening Full`) _returnvalue (struct) 1.0 1.0 0.0 null null null)
    (else
      (`GameplayStatics.PlaySoundAtLocation` (`self.Opening`) _returnvalue (struct) 1.0 1.0 0.0 null null null)))
  (set `self.Close Full` false))

(event `self.Box1.OnComponentBeginOverlap`
  (params (OverlappedComponent :type "PrimitiveComponent Object Reference") (OtherActor :type "Actor Object Reference") (OtherComp :type "PrimitiveComponent Object Reference") (OtherBodyIndex :type Integer) (bFromSweep :type Boolean) (SweepResult :type "HitResult Structure (by ref)"))
  (bind (_returnvalue_location _returnvalue_rotation) (`KismetMathLibrary.BreakTransform` (`SceneComponent.K2_GetComponentToWorld` (`self.In Door`))))
  (bind _asbp_base_ai (cast `/Game/Main/Characters/AI/Neighbor/BP_Base_AI` OtherActor))
  (if (`self.AI Can Open?`)
    (`/Engine/EditorBlueprintResources/StandardMacros.Gate` false :!label _label_6
      (:`Exit`
        (`self.Disable AI Open Door`)
        (set `self.Neighbor` _asbp_base_ai)
        (if (`self.Open`)
          (`self.Delay Close Door`)
          (else
            (set `self.Side` "NewEnumerator1")
            (`/Game/Main/Characters/AI/Neighbor/BP_Base_AI.Lerp Location And Rotation` (`self.Neighbor`) _returnvalue_location _returnvalue_rotation)
            (`/Game/Main/Characters/AI/Neighbor/BP_Base_AI.Set Speed` (`self.Neighbor`) 0.0 :!label _label_7)
            (`KismetSystemLibrary.Delay` 0.2)
            (bind _returnvalue (`Character.PlayAnimMontage` (`self.Neighbor`) "/Game/Main/Characters/Neighbor/Animations/AM_Neighbor_Opening_Door.AM_Neighbor_Opening_Door" 1.0 "None"))
            (`|ExecutionSequence`
              (:`then_0`
                (`KismetSystemLibrary.Delay` _returnvalue)
                (`/Game/Main/Characters/AI/Neighbor/BP_Base_AI.Reset Speed` (`self.Neighbor`)))
              (:`then_1`
                (`KismetSystemLibrary.Delay` 0.7)
                (switch `/Game/Main/Objects/Blueprint/Door/E_Door_Open_Side` (`self.Side`)
                  (:`NewEnumerator0`
                    (`self.Open Door Inward`))
                  (:`NewEnumerator1`
                    (`self.Open Door Outward`)))
                (`KismetSystemLibrary.Delay` 2.0 :!label _label_8)
                (`self.Close Door`)
                (`KismetSystemLibrary.Delay` 1.0)
                (`self.Enable AI Open Door`)))))))))

(event `Enable AI Open Door`
  (bind (_returnvalue_location _returnvalue_rotation) (`KismetMathLibrary.BreakTransform` (`SceneComponent.K2_GetComponentToWorld` (`self.Out Door`))))
  (`|ExecutionSequence`
    (:`then_0`
      (goto _label_6 :!via `Open`))
    (:`then_1`
      (goto _label_9 :!via `Open`))))

(event `Disable AI Open Door`
  (bind (_returnvalue_location _returnvalue_rotation) (`KismetMathLibrary.BreakTransform` (`SceneComponent.K2_GetComponentToWorld` (`self.Out Door`))))
  (`|ExecutionSequence`
    (:`then_0`
      (goto _label_6 :!via `Close`))
    (:`then_1`
      (goto _label_9 :!via `Close`))))

(event `self.Box2.OnComponentBeginOverlap`
  (params (OverlappedComponent :type "PrimitiveComponent Object Reference") (OtherActor :type "Actor Object Reference") (OtherComp :type "PrimitiveComponent Object Reference") (OtherBodyIndex :type Integer) (bFromSweep :type Boolean) (SweepResult :type "HitResult Structure (by ref)"))
  (bind (_returnvalue_location _returnvalue_rotation) (`KismetMathLibrary.BreakTransform` (`SceneComponent.K2_GetComponentToWorld` (`self.Out Door`))))
  (bind _asbp_base_ai (cast `/Game/Main/Characters/AI/Neighbor/BP_Base_AI` OtherActor))
  (if (`self.AI Can Open?`)
    (`/Engine/EditorBlueprintResources/StandardMacros.Gate` false :!label _label_9
      (:`Exit`
        (`self.Disable AI Open Door`)
        (set `self.Neighbor` _asbp_base_ai)
        (if (`self.Open`)
          (`self.Delay Close Door`)
          (else
            (set `self.Side` "NewEnumerator0")
            (`/Game/Main/Characters/AI/Neighbor/BP_Base_AI.Lerp Location And Rotation` (`self.Neighbor`) _returnvalue_location _returnvalue_rotation)
            (goto _label_7)))))))

(event `Delay Close Door`
  (goto _label_8))

(fn `UserConstructionScript`
  (`parent.UserConstructionScript`))