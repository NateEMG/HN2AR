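; BP_Key is a usable key item that opens a BP_Lock_Red whose code matches its own.
; When socket creation runs, it sets its socket to Quentin's Items socket.
; On Use, it runs a short visibility trace through Quentin and casts the hit actor to the lock.
; If the codes match and the lock mesh is not yet simulating physics, it turns physics on to release the lock.
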(event `self.Run Socket Creation`
  (set `self.Socket` (`/Game/Main/Characters/Quentin/Blueprint/CH_Quentin.Items` (`self.Quentin`))))

(event `self.Use`
  (bind (_returnvalue _outhit) (`/Game/Main/Characters/Quentin/Blueprint/CH_Quentin.Trace` (`self.Quentin`) "TraceTypeQuery1" "None" 300.0))
  (if _returnvalue
    (bind _asbp_lock_red (cast `/Game/Main/Objects/Blueprint/BP_Lock_Red` (`.HitActor` (`GameplayStatics.BreakHitResult` _outhit))))
    (if (`SceneComponent.IsSimulatingPhysics` (`/Game/Main/Objects/Blueprint/BP_Base_Item.Mesh` _asbp_lock_red) "None")
      _
      (elif (`KismetStringLibrary.EqualEqual_StrStr` (`/Game/Main/Objects/Blueprint/BP_Lock_Red.Code` _asbp_lock_red) (`self.Code`))
        (`PrimitiveComponent.SetSimulatePhysics` (`/Game/Main/Objects/Blueprint/BP_Base_Item.Mesh` _asbp_lock_red) true)))))

(fn `UserConstructionScript`
  (`parent.UserConstructionScript`))