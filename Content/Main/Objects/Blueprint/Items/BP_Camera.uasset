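; BP_Camera is a camera inventory item that the player character, Quentin, can place in the world.
; Its socket creation event sets Socket to Quentin's Items.
; On Use, a short visibility trace from Quentin finds a surface, where the item is removed from selection and inventory, placed at the impact point facing the player's camera, and given collision again.
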(event `self.Run Socket Creation`
  (set `self.Socket` (`/Game/Main/Characters/Quentin/Blueprint/CH_Quentin.Items` (`self.Quentin`))))

(event `self.Use`
  (bind _quentin (`self.Quentin`))
  (bind (_returnvalue _outhit) (`/Game/Main/Characters/Quentin/Blueprint/CH_Quentin.Trace` (`self.Quentin`) "TraceTypeQuery1" "None" 300.0))
  (if _returnvalue
    (bind (_bblockinghit _binitialoverlap _time _distance _location _impactpoint) (`GameplayStatics.BreakHitResult` _outhit))
    (`/Game/Main/Characters/Quentin/Blueprint/CH_Quentin.Remove Selected Item` _quentin _impactpoint (`KismetMathLibrary.FindLookAtRotation` _impactpoint (`SceneComponent.K2_GetComponentLocation` (`/Game/Main/Characters/Quentin/Blueprint/CH_Quentin.Camera` (`self.Quentin`)))))
    (`/Game/Main/Characters/Quentin/Blueprint/CH_Quentin.Remove From Inventory` _quentin)
    (`self.SetActorEnableCollision` true)))

(fn `UserConstructionScript`
  (`parent.UserConstructionScript`))