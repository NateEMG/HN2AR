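; BP_Binoculars is a droppable item that gives Quentin a zoomed binocular view.
; Use toggles the view, saving the camera's field of view before narrowing it and showing the binocular widget, then restoring both when switched off.
; Drop runs the parent logic and switches off an active view.
; RemoveBinoculars shares that reset path but enters it without checking whether the binoculars are in use.
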(event `self.Use`
  (bind _quentin (`self.Quentin`))
  (bind _binocular_widget (`/Game/Main/Characters/Quentin/Blueprint/CH_Quentin.Binocular Widget` _quentin))
  (if (`self.Using Binoculars`)
    (set `self.Using Binoculars` false)
    (`/Game/Main/Characters/Quentin/Blueprint/CH_Quentin.Set FOV` _quentin (`self.OG FOV`))
    (`Widget.SetVisibility` _binocular_widget "Hidden")
    (else
      (set `self.Using Binoculars` true)
      (set `self.OG FOV` (`CameraComponent.FieldOfView` (`/Game/Main/Characters/Quentin/Blueprint/CH_Quentin.Camera` _quentin)))
      (`/Game/Main/Characters/Quentin/Blueprint/CH_Quentin.Set FOV` (`self.Quentin`) 30.0)
      (`Widget.SetVisibility` _binocular_widget "Visible"))))

(event `Remove Binoculars`
  (set `self.Using Binoculars` false :!label _label)
  (`/Game/Main/Characters/Quentin/Blueprint/CH_Quentin.Set FOV` (`self.Quentin`) (`self.OG FOV`))
  (`Widget.SetVisibility` (`/Game/Main/Characters/Quentin/Blueprint/CH_Quentin.Binocular Widget` (`self.Quentin`)) "Hidden"))

(event `self.Drop`
  (`parent.Drop`)
  (if (`self.Using Binoculars`)
    (goto _label)))

(fn `UserConstructionScript`
  (`parent.UserConstructionScript`))