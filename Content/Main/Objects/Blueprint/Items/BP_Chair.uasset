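; BP_Chair is a chair item whose use action currently only tests for a door in view, with a debug print as placeholder behavior.
; RunSocketCreation sets its Socket from Quentin's Items.
; Use runs a short visibility trace through Quentin and prints "Hello" when the hit component is a BP_Door's Door.
; BeginPlay, overlap, Tick and the construction script add no logic of their own.
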(event `self.Run Socket Creation`
  (set `self.Socket` (`/Game/Main/Characters/Quentin/Blueprint/CH_Quentin.Items` (`self.Quentin`))))

(event `self.Use`
  (bind (_returnvalue _outhit) (`/Game/Main/Characters/Quentin/Blueprint/CH_Quentin.Trace` (`self.Quentin`) "TraceTypeQuery1" "None" 300.0))
  (if _returnvalue
    (bind (_bblockinghit _binitialoverlap _time _distance _location _impactpoint _normal _impactnormal _physmat _hitactor _hitcomponent) (`GameplayStatics.BreakHitResult` _outhit))
    (bind _asbp_door (cast `/Game/Main/Objects/Blueprint/Door/BP_Door` _hitactor))
    (if (== (`/Game/Main/Objects/Blueprint/Door/BP_Door.Door` _asbp_door) _hitcomponent)
      (`KismetSystemLibrary.PrintString` "Hello"))))

(fn `UserConstructionScript`
  (`parent.UserConstructionScript`))