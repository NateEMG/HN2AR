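; Fire extinguisher item that Quentin can pick up, drop and hold to spray.
; Holding use sets Quentin's animation task and starts the particle spray; if he is falling, a short-delayed additive launch along his mesh's up vector gives a small boost.
; Releasing resets the task and stops the spray after a delay.
; Pickup switches the skeletal mesh to Animation Blueprint mode after a delay, and dropping returns it to single-node animation.
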(event `self.Hold Use`
  (bind _quentin (`self.Quentin`))
  (set `/Game/Main/Characters/Quentin/Blueprint/CH_Quentin.Anim Task` "NewEnumerator14" (`self.Quentin`))
  (`ActorComponent.Activate` (`self.ParticleSystem`) false)
  (if (`NavMovementComponent.IsFalling` (`Character.CharacterMovement` _quentin))
    (`KismetSystemLibrary.Delay` 0.1)
    (`Character.LaunchCharacter` (`self.Quentin`) (* (`SceneComponent.GetUpVector` (`Character.Mesh` _quentin)) 80.0) false false)))

(event `self.Stop Hold Use`
  (set `/Game/Main/Characters/Quentin/Blueprint/CH_Quentin.Anim Task` "NewEnumerator15" (`self.Quentin`))
  (`KismetSystemLibrary.Delay` 0.2)
  (set `/Game/Main/Characters/Quentin/Blueprint/CH_Quentin.Anim Task` "NewEnumerator1" (`self.Quentin`))
  (`ActorComponent.Deactivate` (`self.ParticleSystem`)))

(event `/Game/Main/Objects/Blueprint/Base/BP_Base_Item.Pick Up`
  (`parent.Pick Up`)
  (`KismetSystemLibrary.Delay` 0.3)
  (`SkeletalMeshComponent.SetAnimationMode` (`self.SkeletalMesh`) "AnimationBlueprint"))

(event `/Game/Main/Objects/Blueprint/Base/BP_Base_Item.Drop`
  (`parent.Drop`)
  (`SkeletalMeshComponent.SetAnimationMode` (`self.SkeletalMesh`) "AnimationSingleNode"))

(fn `UserConstructionScript`
  (`parent.UserConstructionScript`))