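; BP_Wardrobe is a wardrobe hiding spot for the Quentin character, where interacting with either door calls Hide.
; WardrobeHide switches the doors to Animation Blueprint mode, starts Quentin's animation task, disables collision and control rotation, then locks movement and look after a timed delay.
; WardrobeExit plays the exit task, restores input, movement and collision after a delay, repositions Quentin, shows the item and returns the doors to single-node animation.
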(event `/Game/Main/Characters/Quentin/Blueprint/Interaction_Interface.Interact`
  (params (Component :type "ActorComponent Object Reference"))
  (if (or (== Component (`self.DoorL`)) (== Component (`self.DoorR`)))
    (`self.Hide`)))

(event `self.Wardrobe Hide`
  (`SkeletalMeshComponent.SetAnimationMode` (`self.Doors`) "AnimationBlueprint")
  (`/Game/Main/Characters/Quentin/Blueprint/CH_Quentin.Set Movement Mode` (`self.Quentin`) "MOVE_Flying")
  (`self.SetActorEnableCollision` (`self.Quentin`) false)
  (`/Game/Main/Characters/Quentin/Blueprint/CH_Quentin.Use Control Rotation` (`self.Quentin`) false)
  (set `Pawn.bUseControllerRotationYaw` false (`self.Quentin`))
  (set `/Game/Main/Characters/Quentin/Blueprint/CH_Quentin.Anim Task` "NewEnumerator12" (`self.Quentin`))
  (`KismetSystemLibrary.Delay` 1.7)
  (`self.EnableInput` (`self.Quentin`) (`GameplayStatics.GetPlayerController` 0))
  (`/Game/Main/Objects/HNAR_Function_Library.Set Quentin Movement Mode` "MOVE_None")
  (`/Game/Main/Characters/Quentin/Blueprint/CH_Quentin.Enable / Disable Look` (`self.Quentin`) false))

(event `self.Wardrobe Exit`
  (bind _quentin (`self.Quentin`))
  (`self.DisableInput` _quentin (`GameplayStatics.GetPlayerController` 0))
  (`/Game/Main/Objects/HNAR_Function_Library.Set Quentin Movement Mode` "MOVE_Flying")
  (`/Game/Main/Characters/Quentin/Blueprint/CH_Quentin.Stop / Start Movement` _quentin false)
  (`self.SetActorEnableCollision` (`self.Quentin`) false)
  (`/Game/Main/Characters/Quentin/Blueprint/CH_Quentin.Use Control Rotation` (`self.Quentin`) false)
  (`/Game/Main/Objects/HNAR_Function_Library.Set Quentin Animation Task` "NewEnumerator13")
  (`KismetSystemLibrary.Delay` 1.291)
  (`/Game/Main/Objects/HNAR_Function_Library.Set Quentin Animation Task` "NewEnumerator1")
  (`self.EnableInput` (`self.Quentin`) (`GameplayStatics.GetPlayerController` 0))
  (`/Game/Main/Objects/HNAR_Function_Library.Set Quentin Movement Mode` "MOVE_Walking")
  (`/Game/Main/Characters/Quentin/Blueprint/CH_Quentin.Stop / Start Movement` (`self.Quentin`) true)
  (`self.SetActorEnableCollision` (`self.Quentin`) true)
  (`/Game/Main/Characters/Quentin/Blueprint/CH_Quentin.Use Control Rotation` (`self.Quentin`) true)
  (`/Game/Main/Characters/Quentin/Blueprint/CH_Quentin.Enable / Disable Look` (`self.Quentin`) true)
  (set `Pawn.bUseControllerRotationYaw` true (`self.Quentin`))
  (`/Game/Main/Objects/HNAR_Function_Library.Set Quentin Location and Rotation` (`SceneComponent.K2_GetComponentLocation` (`self.Quentin Location`)) (`SceneComponent.K2_GetComponentRotation` (`self.In Spot`)))
  (`/Game/Main/Characters/Quentin/Blueprint/CH_Quentin.Show Item` (`self.Quentin`))
  (`SkeletalMeshComponent.SetAnimationMode` (`self.Doors`) "AnimationSingleNode"))

(fn `UserConstructionScript`
  (`parent.UserConstructionScript`))