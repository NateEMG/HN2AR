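; Base item actor that supplies shared pick-up and drop behavior for items in the game.
; PickUp turns off mesh physics and actor collision, then plays the pick-up sound at Quentin's location after a short delay.
; Drop restores physics and collision.
; Use and RunSocketCreation are empty events here, and the construction script only calls its parent.
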(event `Run Socket Creation`)

(event `Pick Up`
  (`PrimitiveComponent.SetSimulatePhysics` (`self.Mesh`) false)
  (`self.SetActorEnableCollision` false)
  (`KismetSystemLibrary.Delay` 0.3)
  (`GameplayStatics.PlaySoundAtLocation` (`self.Pick Up Sound`) (`self.K2_GetActorLocation` (`self.Quentin`)) (struct) 1.0 1.0 0.0 null null null))

(event `Drop`
  (`PrimitiveComponent.SetSimulatePhysics` (`self.Mesh`) true)
  (`self.SetActorEnableCollision` true))

(event `Use`)

(fn `UserConstructionScript`
  (`parent.UserConstructionScript`))