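; BP_Lock_Pick is a usable lock pick that opens BP_Lock_Pick_Lock actors by making them physical.
; Its Use event runs a short Visibility trace through the Quentin reference and casts the hit actor to that lock class.
; If the lock's mesh is not already simulating physics, it turns simulation on, with no other unlock state or checks.
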(event `/Game/Main/Objects/Blueprint/Base/BP_Base_Item.Use`
  (bind (_returnvalue _outhit) (`/Game/Main/Characters/Quentin/Blueprint/CH_Quentin.Trace` (`self.Quentin`) "TraceTypeQuery1" "None" 300.0))
  (if _returnvalue
    (bind _asbp_lock_pick_lock (cast `/Game/Main/Objects/Blueprint/BP_Lock_Pick_Lock` (`.HitActor` (`GameplayStatics.BreakHitResult` _outhit))))
    (if (not (`SceneComponent.IsSimulatingPhysics` (`/Game/Main/Objects/Blueprint/Base/BP_Base_Object.Mesh` _asbp_lock_pick_lock) "None"))
      (`PrimitiveComponent.SetSimulatePhysics` (`/Game/Main/Objects/Blueprint/Base/BP_Base_Object.Mesh` _asbp_lock_pick_lock) true))))

(fn `UserConstructionScript`
  (`parent.UserConstructionScript`))