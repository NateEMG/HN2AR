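; Base item actor for physics objects that can be picked up, dropped and used, with Use left as an empty event.
; PickUp turns off mesh physics and actor collision and plays a pickup sound after a short delay, while Drop re-enables both.
; Mesh hits above a speed threshold play an impact sound, throttled by a DoOnce that resets after a delay.
; RunSocketCreation sets the Socket variable from Quentin.Items.
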(event `Run Socket Creation`
  (set `self.Socket` (`/Game/Main/Characters/Quentin/Blueprint/CH_Quentin.Items` (`self.Quentin`))))

(event `Pick Up`
  (`PrimitiveComponent.SetSimulatePhysics` (`self.Mesh`) false)
  (`self.SetActorEnableCollision` false)
  (`KismetSystemLibrary.Delay` 0.3)
  (`GameplayStatics.PlaySoundAtLocation` (`self.Pick Up Sound`) (`self.K2_GetActorLocation`) (struct) 1.0 1.0 0.0 null null null))

(event `Drop`
  (`PrimitiveComponent.SetSimulatePhysics` (`self.Mesh`) true)
  (`self.SetActorEnableCollision` true))

(event `Use`)

(event `self.Mesh.OnComponentHit`
  (params (HitComponent :type "PrimitiveComponent Object Reference") (OtherActor :type "Actor Object Reference") (OtherComp :type "PrimitiveComponent Object Reference") (NormalImpulse :type "Vector Structure") (Hit :type "HitResult Structure (by ref)"))
  (if (>= (`KismetMathLibrary.VSize` (`self.GetVelocity`)) 200.0)
    (`/Engine/EditorBlueprintResources/StandardMacros.DoOnce` false :!label _label
      (:`Completed`
        (`GameplayStatics.PlaySoundAtLocation` (`self.Hit Sound`) (`self.K2_GetActorLocation`) (struct) 1.0 1.0 0.0 null null null)
        (`KismetSystemLibrary.Delay` 0.4)
        (goto _label :!via `Reset`)))))

(fn `UserConstructionScript`
  (`parent.UserConstructionScript`))