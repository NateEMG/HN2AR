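; BP_Clock is a clock object Blueprint that can play a clock noise at its own location.
; On BeginPlay it rolls a random integer, and only on a zero does it play the attenuated sound cue, wait briefly and roll again.
; Any non-zero roll ends the chain, so most instances stay silent.
; The overlap event is disabled and the construction script only calls its parent.
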(event `self.ReceiveBeginPlay`
  (`parent.ReceiveBeginPlay`)
  (if (== (`KismetMathLibrary.RandomIntegerInRange` 0 50) 0) :!label _label
    (`GameplayStatics.PlaySoundAtLocation` "/Game/Main/Sounds/HN2SoundBank/clock_noise_Cue.clock_noise_Cue" (`self.K2_GetActorLocation`) (struct) 1.0 1.0 0.0 "/Game/Main/Sounds/Main.Main" null null)
    (`KismetSystemLibrary.Delay` 0.5)
    (goto _label)))

(fn `UserConstructionScript`
  (`parent.UserConstructionScript`))