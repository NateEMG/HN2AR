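; Base object Blueprint that switches its visible representation between a Mesh component and a SkeletalMesh component.
; RunSkeletalCreation shows the SkeletalMesh and hides Mesh, while RunSkeletalDeletion does the reverse.
; The swap only toggles visibility without propagating to children, so no component is actually created or destroyed.
; BeginPlay, overlap and Tick are disabled stubs, and the construction script only calls its parent.
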(event `self.Run Skeletal Deletion`
  (`SceneComponent.SetVisibility` (`self.Mesh`) true false)
  (`SceneComponent.SetVisibility` (`self.SkeletalMesh`) false false))

(event `self.Run Skeletal Creation`
  (`SceneComponent.SetVisibility` (`self.Mesh`) false false)
  (`SceneComponent.SetVisibility` (`self.SkeletalMesh`) true false))

(fn `UserConstructionScript`
  (`parent.UserConstructionScript`))