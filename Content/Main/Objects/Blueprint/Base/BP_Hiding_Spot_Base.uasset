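; Base hiding spot Blueprint that toggles Quentin in and out of hiding through a Hide event.
; Entry requires a specific AnimTask state, uncrouches Quentin, disables input and movement, hides the held item and lerps to an approach point.
; Regular spots then snap Quentin inside with a sound, and teleport back to that point on exit.
; Wardrobe spots instead call empty WardrobeHide and WardrobeExit events.
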(event `Wardrobe Exit`)

(event `Wardrobe Hide`)

(event `Hide`
  (bind _quentin (`self.Quentin`))
  (bind _quentin_2 (`self.Quentin`))
  (bind (_returnvalue_location _returnvalue_rotation) (`KismetMathLibrary.BreakTransform` (`SceneComponent.K2_GetComponentToWorld` (`self.In Spot`))))
  (bind (_returnvalue_location_2 _returnvalue_rotation_2) (`KismetMathLibrary.BreakTransform` (`SceneComponent.K2_GetComponentToWorld` (`self.Quentin Location`))))
  (if (`|EnumEquality` (`CharacterMovementComponent.MovementMode` (`Character.CharacterMovement` (`self.Quentin`))) "MOVE_Flying")
    _
    (elif (`/Game/Main/Characters/Quentin/Blueprint/CH_Quentin.Hiding` _quentin)
      (set `/Game/Main/Characters/Quentin/Blueprint/CH_Quentin.Hiding` false (`self.Quentin`))
      (if (`self.Wardrobe`)
        (`self.Wardrobe Exit`)
        (else
          (`self.K2_SetActorLocation` (`self.Quentin`) (`SceneComponent.K2_GetComponentLocation` (`self.Quentin Location`)) false false)))
      (elif (`|EnumEquality` (`/Game/Main/Characters/Quentin/Blueprint/CH_Quentin.Anim Task` _quentin) "NewEnumerator1")
        (set `/Game/Main/Characters/Quentin/Blueprint/CH_Quentin.Hiding` true _quentin_2)
        (if (`NavMovementComponent.IsCrouching` (`Character.CharacterMovement` _quentin_2))
          (`Character.UnCrouch` (`self.Quentin`))
          (`KismetSystemLibrary.Delay` 0.2))
        (`self.DisableInput` (`self.Quentin`) (`GameplayStatics.GetPlayerController` 0))
        (`/Game/Main/Characters/Quentin/Blueprint/CH_Quentin.Hide Item` (`self.Quentin`))
        (`/Game/Main/Objects/HNAR_Function_Library.Set Quentin Movement Mode` "MOVE_None")
        (`/Game/Main/Characters/Quentin/Blueprint/CH_Quentin.Stop / Start Movement` (`self.Quentin`) false)
        (`/Game/Main/Characters/Quentin/Blueprint/CH_Quentin.Lerp Location` (`self.Quentin`) _returnvalue_location_2)
        (`/Game/Main/Characters/Quentin/Blueprint/CH_Quentin.Lerp Rotation` (`self.Quentin`) _returnvalue_rotation_2)
        (`KismetSystemLibrary.Delay` 0.3)
        (if (`self.Wardrobe`)
          (`self.Wardrobe Hide`)
          (else
            (`/Game/Main/Objects/HNAR_Function_Library.Set Quentin Location and Rotation` _returnvalue_location _returnvalue_rotation)
            (`GameplayStatics.PlaySoundAtLocation` (`self.Hide Sound`) (`self.K2_GetActorLocation`) (struct) 1.0 1.0 0.0 "/Game/Main/Sounds/Main.Main" null null)))))))

(fn `UserConstructionScript`)