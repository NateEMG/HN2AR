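; BP_TV_Stand is a TV stand prop with two doors that swing open and closed on interaction.
; Interact checks which door component is passed in and flips that side's open flag to call its open or close event.
; Each event rotates the door's yaw with Move Component To, first calling a shared Stop that halts all four moves, including the other door's.
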(event `/Game/Main/Characters/Quentin/Blueprint/Interaction_Interface.Interact`
  (params (Component :type "ActorComponent Object Reference"))
  (if (== Component (`self.dresser1door`))
    (if (`self.Open L`)
      (set `self.Open L` false)
      (`self.Close L`)
      (else
        (set `self.Open L` true)
        (`self.OpenL`)))
    (elif (== Component (`self.dresser1door1`))
      (if (`self.Open R`)
        (set `self.Open R` false)
        (`self.Close R`)
        (else
          (set `self.Open R` true)
          (`self.OpenR`))))))

(event `Close L`
  (bind _dresser1door (`self.dresser1door`))
  (bind (_relativerotation_roll _relativerotation_pitch) (`KismetMathLibrary.BreakRotator` (`SceneComponent.RelativeRotation` _dresser1door)))
  (`self.Stop`)
  (`KismetSystemLibrary.MoveComponentTo` _dresser1door (`SceneComponent.RelativeLocation` _dresser1door) (`KismetMathLibrary.MakeRotator` _relativerotation_roll _relativerotation_pitch) false false 0.2 true :!label _label))

(event `Close R`
  (bind _dresser1door1 (`self.dresser1door1`))
  (bind (_relativerotation_roll _relativerotation_pitch) (`KismetMathLibrary.BreakRotator` (`SceneComponent.RelativeRotation` _dresser1door1)))
  (`self.Stop`)
  (`KismetSystemLibrary.MoveComponentTo` _dresser1door1 (`SceneComponent.RelativeLocation` _dresser1door1) (`KismetMathLibrary.MakeRotator` _relativerotation_roll _relativerotation_pitch 0.0) false false 0.2 true :!label _label_2))

(event `Stop`
  (bind _dresser1door (`self.dresser1door`))
  (bind _dresser1door1 (`self.dresser1door1`))
  (bind (_relativerotation_roll _relativerotation_pitch) (`KismetMathLibrary.BreakRotator` (`SceneComponent.RelativeRotation` _dresser1door1)))
  (bind (_relativerotation_roll_2 _relativerotation_pitch_2) (`KismetMathLibrary.BreakRotator` (`SceneComponent.RelativeRotation` _dresser1door)))
  (`|ExecutionSequence`
    (:`then_0`
      (goto _label :!via `Stop`))
    (:`then_1`
      (goto _label_2 :!via `Stop`))
    (:`then_2`
      (goto _label_4 :!via `Stop`))
    (:`then_3`
      (goto _label_3 :!via `Stop`))))

(event `OpenL`
  (bind _dresser1door (`self.dresser1door`))
  (bind (_relativerotation_roll _relativerotation_pitch) (`KismetMathLibrary.BreakRotator` (`SceneComponent.RelativeRotation` _dresser1door)))
  (`self.Stop`)
  (`KismetSystemLibrary.MoveComponentTo` _dresser1door (`SceneComponent.RelativeLocation` _dresser1door) (`KismetMathLibrary.MakeRotator` _relativerotation_roll _relativerotation_pitch 100.0) false false 0.2 true :!label _label_3))

(event `OpenR`
  (bind _dresser1door1 (`self.dresser1door1`))
  (bind (_relativerotation_roll _relativerotation_pitch) (`KismetMathLibrary.BreakRotator` (`SceneComponent.RelativeRotation` _dresser1door1)))
  (`self.Stop`)
  (`KismetSystemLibrary.MoveComponentTo` _dresser1door1 (`SceneComponent.RelativeLocation` _dresser1door1) (`KismetMathLibrary.MakeRotator` _relativerotation_roll _relativerotation_pitch -100.0) false false 0.2 true :!label _label_4))

(fn `UserConstructionScript`
  (`parent.UserConstructionScript`))