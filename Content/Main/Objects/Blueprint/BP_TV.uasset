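; BP_TV is an interactable television that the player or a neighbor can toggle on and off.
; Interact fires only on the switch mesh and shares NeighborInteract's toggle, which plays an on/off sound and rotates the switch with paired MoveComponentTo nodes, stopping the opposing move.
; When Powered, SwitchOn and SwitchOff swap the screen material between a landscape picture and glass, and start or stop the looping TV audio.
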(event `/Game/Main/Objects/Blueprint/Base/BP_Base_Object.Neighbor Interact`
  (params (Neighbor :type "/Game/Main/Characters/AI/Neighbor/BP_Base_AI Object Reference"))
  (bind _returnvalue (`self.K2_GetActorLocation`))
  (bind _o_sm_hideouttv_switch_lod0_mo (`self.O_SM_HideoutTV_Switch_LOD0_mo`))
  (bind _relativelocation (`SceneComponent.RelativeLocation` _o_sm_hideouttv_switch_lod0_mo))
  (if (`self.Switched On`) :!label _label
    (set `self.Switched On` false)
    (`self.Switch Off`)
    (`GameplayStatics.PlaySoundAtLocation` "/Game/Main/Sounds/HN2SoundBank/tv_off_Cue.tv_off_Cue" _returnvalue (struct) 1.0 1.0 0.0 null null null)
    (`|ExecutionSequence`
      (:`then_0`
        (goto _label_3 :!via `Stop`))
      (:`then_1`
        (`KismetSystemLibrary.MoveComponentTo` _o_sm_hideouttv_switch_lod0_mo _relativelocation (struct) false false 0.2 true :!label _label_2)))
    (else
      (set `self.Switched On` true)
      (`self.Switch On`)
      (`GameplayStatics.PlaySoundAtLocation` "/Game/Main/Sounds/HN2SoundBank/tv_on_Cue.tv_on_Cue" _returnvalue (struct) 1.0 1.0 0.0 null null null)
      (`|ExecutionSequence`
        (:`then_0`
          (goto _label_2 :!via `Stop`))
        (:`then_1`
          (`KismetSystemLibrary.MoveComponentTo` _o_sm_hideouttv_switch_lod0_mo _relativelocation (struct :`Pitch` -40.0) false false 0.2 true :!label _label_3))))))

(event `/Game/Main/Characters/Quentin/Blueprint/Interaction_Interface.Interact`
  (params (Component :type "ActorComponent Object Reference"))
  (if (== Component (`self.O_SM_HideoutTV_Switch_LOD0_mo`))
    (goto _label)))

(event `Switch Off`
  (if (`self.Powered`)
    (`PrimitiveComponent.SetMaterial` (`self.H_SM_TV_01_LOD0_mo`) 1 "/Game/Main/Objects/Items/Meshes/Materials/MI_Glass_01_Inst.MI_Glass_01_Inst")
    (`AudioComponent.Stop` (`self.TV_relax_loop_Cue`))))

(event `Switch On`
  (if (`self.Powered`)
    (`PrimitiveComponent.SetMaterial` (`self.H_SM_TV_01_LOD0_mo`) 1 "/Game/Main/Objects/LocationProps/Hideout/Materials/MI_LandscapePicture.MI_LandscapePicture")
    (`AudioComponent.Play` (`self.TV_relax_loop_Cue`) 0.0)))

(fn `UserConstructionScript`
  (`parent.UserConstructionScript`))