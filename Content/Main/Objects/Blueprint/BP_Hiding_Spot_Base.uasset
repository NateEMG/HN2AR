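; BP_Hiding_Spot_Base is the base Blueprint for spots where the player character Quentin hides.
; Hide disables Quentin's input and movement, then lerps Quentin to the QuentinLocation point.
; After a short delay, a Wardrobe flag routes to the WardrobeHide event, empty here; otherwise Quentin snaps to InSpot and a hide sound plays.
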(event `Wardrobe Hide`)

(event `Hide`
  (bind (_returnvalue_location _returnvalue_rotation) (`KismetMathLibrary.BreakTransform` (`SceneComponent.K2_GetComponentToWorld` (`self.In Spot`))))
  (bind (_returnvalue_location_2 _returnvalue_rotation_2) (`KismetMathLibrary.BreakTransform` (`SceneComponent.K2_GetComponentToWorld` (`self.Quentin Location`))))
  (`self.DisableInput` (`self.Quentin`) (`GameplayStatics.GetPlayerController` 0))
  (`/Game/Main/Objects/HNAR_Function_Library.Set Quentin Movement Mode` "MOVE_None")
  (`/Game/Main/Characters/Quentin/Blueprint/CH_Quentin.Stop / Start Movement` (`self.Quentin`) false)
  (`/Game/Main/Characters/Quentin/Blueprint/CH_Quentin.Lerp Location` (`self.Quentin`) _returnvalue_location_2)
  (`/Game/Main/Characters/Quentin/Blueprint/CH_Quentin.Lerp Rotation` (`self.Quentin`) _returnvalue_rotation_2)
  (`KismetSystemLibrary.Delay` 0.5)
  (if (`self.Wardrobe`)
    (`self.Wardrobe Hide`)
    (else
      (`/Game/Main/Objects/HNAR_Function_Library.Set Quentin Location and Rotation` _returnvalue_location _returnvalue_rotation)
      (`GameplayStatics.PlaySoundAtLocation` (`self.Hide Sound`) (`self.K2_GetActorLocation`) (struct) 1.0 1.0 0.0 "/Game/Main/Sounds/Main.Main" null null))))

(fn `UserConstructionScript`)