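; BP_Ferris_Wheel is a park Ferris wheel actor that continuously spins its static mesh around the pitch axis.
; BeginPlay calls a Rotate event that re-registers itself on a short looping timer with every call, so Tick is unused.
; Each call nudges the mesh's relative pitch up slightly, zeroing roll and yaw, and resets pitch to zero only on an exact float match with 90 degrees.
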(event `self.ReceiveBeginPlay`
  (`self.Rotate`))

(event `Rotate`
  (bind (_relativerotation_roll _relativerotation_pitch) (`KismetMathLibrary.BreakRotator` (`SceneComponent.RelativeRotation` (`self.StaticMesh`))))
  (`KismetSystemLibrary.K2_SetTimerDelegate` (delegate `Rotate`) 0.01 true)
  (if (== _relativerotation_pitch 90.0)
    (`SceneComponent.K2_SetRelativeRotation` (`self.StaticMesh`) (`KismetMathLibrary.MakeRotator` 0.0) false false)
    (else
      (`SceneComponent.K2_SetRelativeRotation` (`self.StaticMesh`) (`KismetMathLibrary.MakeRotator` 0.0 (+ _relativerotation_pitch 0.03)) false false))))

(fn `UserConstructionScript`)