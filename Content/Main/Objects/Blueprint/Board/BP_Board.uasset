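; BP_Board is a board object that can hold a referenced Door locked until the board comes loose.
; With a valid Door, its begin hook disables mesh physics and pickup and locks the door.
; Tick polls the mesh's physics state, keeping the door locked while physics is off and unlocking it through a DoOnce when physics starts, re-armed whenever physics stops.
; A socket-creation hook assigns Quentin's Items as its Socket.
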(event `self.ReceiveTick`
  (params (DeltaSeconds :type "Float (single-precision)"))
  (`/Engine/EditorBlueprintResources/StandardMacros.IsValid` (`self.Door`)
    (:`Is Valid`
      (if (`SceneComponent.IsSimulatingPhysics` (`self.Mesh`) "None")
        (`/Engine/EditorBlueprintResources/StandardMacros.DoOnce` false :!label _label
          (:`Completed`
            (set `/Game/Main/Objects/Blueprint/Door/BP_Door.Locked` false (`self.Door`))))
        (else
          (set `/Game/Main/Objects/Blueprint/Door/BP_Door.Locked` true (`self.Door`))
          (goto _label :!via `Reset`))))))

(event `self.Run Socket Creation`
  (set `self.Socket` (`/Game/Main/Characters/Quentin/Blueprint/CH_Quentin.Items` (`self.Quentin`))))

(event `self.Run Begin Function`
  (`/Engine/EditorBlueprintResources/StandardMacros.IsValid` (`self.Door`)
    (:`Is Valid`
      (`PrimitiveComponent.SetSimulatePhysics` (`self.Mesh`) false)
      (set `self.Can Pick Up` false)
      (set `/Game/Main/Objects/Blueprint/Door/BP_Door.Locked` true (`self.Door`)))))

(fn `UserConstructionScript`
  (`parent.UserConstructionScript`))