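; BP_Radio is an interactable radio actor that plays a music soundtrack cue.
; Interact branches on the On flag: when off, it sets the flag and assigns the radio cue to the Audio component.
; When on, it clears the flag and destroys that component.
; A DoOnce with no reset guards the switch-on path, so the radio can be turned on only once.
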(event `/Game/Main/Characters/Quentin/Blueprint/Interaction_Interface.Interact`
  (params (Component :type "ActorComponent Object Reference"))
  (if (`self.On`)
    (set `self.On` false)
    (`ActorComponent.K2_DestroyComponent` (`self.Audio`))
    (else
      (`/Engine/EditorBlueprintResources/StandardMacros.DoOnce` false
        (:`Completed`
          (set `self.On` true)
          (`AudioComponent.SetSound` (`self.Audio`) "/Game/Main/Sounds/Music/HN2_Music_Radio_OST_Cue.HN2_Music_Radio_OST_Cue"))))))

(fn `UserConstructionScript`
  (`parent.UserConstructionScript`))