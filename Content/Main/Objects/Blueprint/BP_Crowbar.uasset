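; Crowbar item that the Quentin character uses to pry boards loose, attaching to the character's Items socket.
; On hold-use, it traces for a non-simulating BP_Board, registers itself as the interact object and sets an animation task by board state.
; Weak boards get a brief animation task, while strong boards hold theirs until use stops.
; RunInteraction then enables the board's physics and makes it pickable.
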(event `self.Run Socket Creation`
  (set `self.Socket` (`/Game/Main/Characters/Quentin/Blueprint/CH_Quentin.Items` (`self.Quentin`))))

(event `self.Hold Use`
  (bind (_returnvalue _outhit) (`/Game/Main/Characters/Quentin/Blueprint/CH_Quentin.Trace` (`self.Quentin`) "TraceTypeQuery1" "None" 300.0))
  (if _returnvalue
    (bind _asbp_board (cast `/Game/Main/Objects/Blueprint/Board/BP_Board` (`.HitActor` (`GameplayStatics.BreakHitResult` _outhit))))
    (bind _output_get (set `self.Board` _asbp_board))
    (if (not (`SceneComponent.IsAnySimulatingPhysics` (`/Game/Main/Objects/Blueprint/BP_Base_Object.Mesh` _output_get)))
      (set `/Game/Main/Characters/Quentin/Blueprint/CH_Quentin.Interact Object` self (`self.Quentin`))
      (switch `/Game/Main/Objects/Blueprint/Board/E_Board_State` (`/Game/Main/Objects/Blueprint/Board/BP_Board.State` (`self.Board`))
        (:`NewEnumerator0`
          (`self.Break Weak Board`))
        (:`NewEnumerator1`
          (`self.Break Strong Board`))))))

(event `Break Strong Board`
  (bind _quentin (`self.Quentin`))
  (`/Game/Main/Characters/Quentin/Blueprint/CH_Quentin.Enable / Disable Look` _quentin false)
  (set `/Game/Main/Characters/Quentin/Blueprint/CH_Quentin.Anim Task` "NewEnumerator6" _quentin))

(event `self.Stop Hold Use`
  (if (`|EnumEquality` (`/Game/Main/Characters/Quentin/Blueprint/CH_Quentin.Anim Task` (`self.Quentin`)) "NewEnumerator6")
    (set `/Game/Main/Characters/Quentin/Blueprint/CH_Quentin.Anim Task` "NewEnumerator1" (`self.Quentin`))))

(event `Break Weak Board`
  (set `/Game/Main/Characters/Quentin/Blueprint/CH_Quentin.Anim Task` "NewEnumerator4" (`self.Quentin`))
  (`KismetSystemLibrary.Delay` 0.2)
  (set `/Game/Main/Characters/Quentin/Blueprint/CH_Quentin.Anim Task` "NewEnumerator1" (`self.Quentin`)))

(event `self.Run Interaction`
  (set `/Game/Main/Characters/Quentin/Blueprint/CH_Quentin.Interact Object` null (`self.Quentin`))
  (`PrimitiveComponent.SetSimulatePhysics` (`/Game/Main/Objects/Blueprint/BP_Base_Object.Mesh` (`self.Board`)) true)
  (set `/Game/Main/Objects/Blueprint/BP_Base_Item.Can Pick Up` true (`self.Board`))
  (set `self.Board` null))

(fn `UserConstructionScript`
  (`parent.UserConstructionScript`))