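; Trigger volume that plays a level sequence cutscene when CH_Quentin overlaps its box and it is not disabled.
; It creates a sequence player, moves Quentin to the world origin, and waits out the sequence's duration with a Delay.
; It then places Quentin at NewPlayerTransform and applies that rotation to player controller 0.
; The DoOnce branch has nothing wired to Completed, so it does not gate playback.
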(event `self.Box.OnComponentBeginOverlap`
  (params (OverlappedComponent :type "PrimitiveComponent Object Reference") (OtherActor :type "Actor Object Reference") (OtherComp :type "PrimitiveComponent Object Reference") (OtherBodyIndex :type Integer) (bFromSweep :type Boolean) (SweepResult :type "HitResult Structure (by ref)"))
  (bind (_new_player_transform_location _new_player_transform_rotation) (`KismetMathLibrary.BreakTransform` (`self.New Player Transform`)))
  (bind _asch_quentin (cast `/Game/Main/Characters/Quentin/Blueprint/CH_Quentin` OtherActor))
  (if (not (`self.Disabled?`))
    (if (`self.Do Once?`)
      (`/Engine/EditorBlueprintResources/StandardMacros.DoOnce` false
        (:`Completed`
          _)))
    (bind (_outactor _returnvalue) (`LevelSequencePlayer.CreateLevelSequencePlayer` (`self.Cutscene`)))
    (`MovieSceneSequencePlayer.Play` _returnvalue)
    (`self.K2_SetActorLocation` _asch_quentin (0.0 0.0 0.0) false false)
    (`KismetSystemLibrary.Delay` (`TimeManagementBlueprintLibrary.Conv_QualifiedFrameTimeToSeconds` (`MovieSceneSequencePlayer.GetDuration` _returnvalue)))
    (`self.K2_SetActorLocation` _asch_quentin _new_player_transform_location false false)
    (`Controller.SetControlRotation` (`GameplayStatics.GetPlayerController` 0) _new_player_transform_rotation)))

(fn `UserConstructionScript`)