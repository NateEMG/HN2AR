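; BP_Window_Openable is an interactable window that slides open and lets Quentin climb through from either side.
; Interacting with the Moving component raises it via MoveComponentTo, and Quentin leaving the Box lowers it again.
; MoveQuentin checks his AnimTask and overlap with BoxA or BoxB, then snaps him to that side's marker.
; It plays the through-window montage with collision off in Flying mode, guarded by resettable DoOnce gates.
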(event `/Game/Main/Characters/Quentin/Blueprint/Interaction_Interface.Interact`
  (params (Component :type "ActorComponent Object Reference"))
  (if (== Component (`self.Moving`))
    (if (not (`self.Open`))
      (set `self.Open` true)
      (`self.Move Window Up`))))

(event `Move Window Up`
  (bind _moving (`self.Moving`))
  (bind (_relativelocation_x _relativelocation_y) (`KismetMathLibrary.BreakVector` (`SceneComponent.RelativeLocation` _moving)))
  (`KismetSystemLibrary.MoveComponentTo` _moving (`KismetMathLibrary.MakeVector` _relativelocation_x _relativelocation_y 5.0) (`SceneComponent.RelativeRotation` _moving) false false 0.5 true))

(event `Close Window`
  (bind _moving (`self.Moving`))
  (bind (_relativelocation_x _relativelocation_y) (`KismetMathLibrary.BreakVector` (`SceneComponent.RelativeLocation` _moving)))
  (`KismetSystemLibrary.MoveComponentTo` _moving (`KismetMathLibrary.MakeVector` _relativelocation_x _relativelocation_y -105.0) (`SceneComponent.RelativeRotation` _moving) false false 0.5 true))

(event `self.Box.OnComponentEndOverlap`
  (params (OverlappedComponent :type "PrimitiveComponent Object Reference") (OtherActor :type "Actor Object Reference") (OtherComp :type "PrimitiveComponent Object Reference") (OtherBodyIndex :type Integer))
  (cast `/Game/Main/Characters/Quentin/Blueprint/CH_Quentin` OtherActor)
  (if (`self.Open`)
    (set `self.Open` false)
    (`self.Close Window`)))

(event `Move Quentin`
  (bind _quentin (`self.Quentin`))
  (bind (_returnvalue_location _returnvalue_rotation) (`KismetMathLibrary.BreakTransform` (`SceneComponent.K2_GetComponentToWorld` (`self.Open Loc B`))))
  (bind (_returnvalue_location_2 _returnvalue_rotation_2) (`KismetMathLibrary.BreakTransform` (`SceneComponent.K2_GetComponentToWorld` (`self.Open Loc A`))))
  (if (`|EnumEquality` (`/Game/Main/Characters/Quentin/Blueprint/CH_Quentin.Anim Task` (`self.Quentin`)) "NewEnumerator1")
    (if (`PrimitiveComponent.IsOverlappingActor` (`self.Box A`) _quentin)
      (`/Engine/EditorBlueprintResources/StandardMacros.DoOnce` false :!label _label
        (:`Completed`
          (`/Game/Main/Objects/HNAR_Function_Library.Set Quentin Location and Rotation` _returnvalue_location_2 _returnvalue_rotation_2)
          (`self.SetActorEnableCollision` (`self.Quentin`) false :!label _label_2)
          (`/Game/Main/Objects/HNAR_Function_Library.Set Quentin Movement Mode` "MOVE_Flying")
          (bind _delay (`/Game/Main/Objects/HNAR_Function_Library.Play Quentin Montage` "/Game/Main/Characters/Quentin/Animations/AM_Quentin_Through_Window.AM_Quentin_Through_Window"))
          (`KismetSystemLibrary.Delay` _delay)
          (`self.SetActorEnableCollision` (`self.Quentin`) true)
          (`/Game/Main/Objects/HNAR_Function_Library.Set Quentin Movement Mode` "MOVE_Walking")))
      (elif (`PrimitiveComponent.IsOverlappingActor` (`self.Box B`) _quentin)
        (`/Engine/EditorBlueprintResources/StandardMacros.DoOnce` false :!label _label_3
          (:`Completed`
            (`/Game/Main/Objects/HNAR_Function_Library.Set Quentin Location and Rotation` _returnvalue_location _returnvalue_rotation)
            (goto _label_2)))))))

(event `Reset`
  (`|ExecutionSequence`
    (:`then_0`
      (goto _label :!via `Reset`))
    (:`then_1`
      (goto _label_3 :!via `Reset`))))

(fn `UserConstructionScript`)