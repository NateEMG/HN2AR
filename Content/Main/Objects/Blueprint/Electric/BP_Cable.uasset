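; BP_Cable is an electrical object that runs a rope cable between a plug and itself when used.
; Its Use event calls a short visibility trace on Quentin and checks whether the hit component carries the Plug tag.
; On a match, it spawns a BP_Rope_Cable at that component's location and rotation, then attaches the cable's end to its own Cube component.
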(event `/Game/Main/Objects/Blueprint/Base/BP_Base_Item.Use`
  (bind (_returnvalue _outhit) (`/Game/Main/Characters/Quentin/Blueprint/CH_Quentin.Trace` (`self.Quentin`) "TraceTypeQuery1" "None" 300.0))
  (if _returnvalue
    (bind (_bblockinghit _binitialoverlap _time _distance _location _impactpoint _normal _impactnormal _physmat _hitactor _hitcomponent) (`GameplayStatics.BreakHitResult` _outhit))
    (if (`ActorComponent.ComponentHasTag` _hitcomponent "Plug")
      (bind (_returnvalue_location _returnvalue_rotation) (`KismetMathLibrary.BreakTransform` (`SceneComponent.K2_GetComponentToWorld` _hitcomponent)))
      (bind _returnvalue_2 (`|SpawnActorFromClass` "/Game/Main/Objects/Blueprint/Electric/BP_Rope_Cable.BP_Rope_Cable_C" (`KismetMathLibrary.MakeTransform` _returnvalue_location _returnvalue_rotation) "Undefined" "OverrideRootScale" null null))
      (`CableComponent.SetAttachEndToComponent` (`/Game/Main/Objects/Blueprint/Electric/BP_Rope_Cable.Cable` _returnvalue_2) (`self.Cube`) "None"))))

(fn `UserConstructionScript`
  (`parent.UserConstructionScript`))