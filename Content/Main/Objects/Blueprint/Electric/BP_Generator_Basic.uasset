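; BP_Generator_Basic is an interactable electric generator with a part that toggles it on and off.
; Interact on that part flips On and rotates it between two poses over a short timed move, stopping any move in the opposite direction.
; When a move completes and Powered is true, PowerOn or PowerOff swaps the main mesh's red indicator material and the start-loop or stop sound is set.
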(event `/Game/Main/Characters/Quentin/Blueprint/Interaction_Interface.Interact`
  (params (Component :type "ActorComponent Object Reference"))
  (bind _sm_sm_generator_part_01_mo (`self.SM_SM_Generator_Part_01_mo`))
  (bind _relativelocation (`SceneComponent.RelativeLocation` _sm_sm_generator_part_01_mo))
  (if (== Component (`self.SM_SM_Generator_Part_01_mo`))
    (if (`self.On`)
      (`|ExecutionSequence`
        (:`then_0`
          (goto _label_2 :!via `Stop`))
        (:`then_1`
          (set `self.On` false)
          (`KismetSystemLibrary.MoveComponentTo` _sm_sm_generator_part_01_mo _relativelocation (struct) false false 0.5 true :!label _label)
          (if (`self.Powered`)
            (`self.Power Off`)
            (`AudioComponent.SetSound` (`self.Audio`) "/Game/Main/Sounds/HN2SoundBank/Generator_Stop_Cue.Generator_Stop_Cue"))))
      (else
        (`|ExecutionSequence`
          (:`then_0`
            (goto _label :!via `Stop`))
          (:`then_1`
            (set `self.On` true)
            (`KismetSystemLibrary.MoveComponentTo` _sm_sm_generator_part_01_mo _relativelocation (struct :`Roll` 50.0) false false 0.5 true :!label _label_2)
            (if (`self.Powered`)
              (`self.Power On`)
              (`AudioComponent.SetSound` (`self.Audio`) "/Game/Main/Sounds/HN2SoundBank/Generator_Start_Loop_Cue.Generator_Start_Loop_Cue")
              (`AudioComponent.Play` (`self.Audio`) 0.0))))))))

(event `Power On`
  (`PrimitiveComponent.SetMaterial` (`self.O_SM_Generator_01_Main_LOD0_mo`) 0 "/Game/Main/Objects/Special/Materials/MI_Emissive_Red.MI_Emissive_Red"))

(event `Power Off`
  (`PrimitiveComponent.SetMaterial` (`self.O_SM_Generator_01_Main_LOD0_mo`) 0 "/Game/Main/Objects/Special/Materials/MI_Red_OFF.MI_Red_OFF"))

(fn `UserConstructionScript`
  (`parent.UserConstructionScript`))