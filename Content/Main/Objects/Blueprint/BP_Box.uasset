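; BP_Box is a box object Blueprint that extends a parent class, with an option to start hanging.
; On BeginPlay it runs the parent logic, then turns off physics simulation on its Mesh when Hang is set.
; The RunSocketCreation event sets Socket to Quentin.Box.
; Tick and the construction script only call the parent.
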(event `self.ReceiveBeginPlay`
  (`parent.ReceiveBeginPlay`)
  (if (`self.hang?`)
    (`PrimitiveComponent.SetSimulatePhysics` (`self.Mesh`) false)))

(event `self.ReceiveTick`
  (params (DeltaSeconds :type "Float (single-precision)"))
  (`parent.ReceiveTick` DeltaSeconds))

(event `self.Run Socket Creation`
  (set `self.Socket` (`/Game/Main/Characters/Quentin/Blueprint/CH_Quentin.Box` (`self.Quentin`))))

(fn `UserConstructionScript`
  (`parent.UserConstructionScript`))