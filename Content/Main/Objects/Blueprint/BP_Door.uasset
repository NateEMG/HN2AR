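; Interactive hinged door that plays a lock sound when locked and otherwise toggles open and closed when its Door component is interacted with.
; Opening checks whether Quentin overlaps the Box to choose which of two opposite directions to swing.
; MoveComponentTo drives each swing, stopping opposing moves so the door can reverse midway.
; Closing audio plays during the return and fades into a closed sound on completion.
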(event `/Game/Main/Characters/Quentin/Blueprint/Interaction_Interface.Interact`
  (params (Component :type "ActorComponent Object Reference"))
  (bind _door (`self.Door`))
  (bind _relativelocation (`SceneComponent.RelativeLocation` _door))
  (if (== Component (`self.Door`))
    (if (`self.Locked`)
      (`GameplayStatics.PlaySoundAtLocation` (`self.Lock`) (`SceneComponent.K2_GetComponentLocation` (`self.Door`)) (struct) 1.0 1.0 0.0 null null null)
      (elif (`self.Open`)
        (`|ExecutionSequence`
          (:`then_0`
            (goto _label_3 :!via `Stop`))
          (:`then_1`
            (goto _label_2 :!via `Stop`))
          (:`then_2`
            (set `self.Open` false)
            (`AudioComponent.Play` (`self.Closing Audio`) 0.0)
            (`KismetSystemLibrary.MoveComponentTo` _door _relativelocation (struct) false false (`self.Over Time`) true :!label _label)
            (`AudioComponent.FadeOut` (`self.Closing Audio`) 0.2 0.0 "Linear")
            (`GameplayStatics.PlaySoundAtLocation` (`self.Closed`) (`SceneComponent.K2_GetComponentLocation` (`self.Door`)) (struct) 1.0 1.0 0.0 null null null)))
        (else
          (`|ExecutionSequence`
            (:`then_0`
              (goto _label :!via `Stop`))
            (:`then_1`
              (set `self.Open` true)
              (`GameplayStatics.PlaySoundAtLocation` (`self.Opening`) (`SceneComponent.K2_GetComponentLocation` (`self.Door`)) (struct) 1.0 1.0 0.0 null null null)
              (if (`PrimitiveComponent.IsOverlappingActor` (`self.Box`) (`self.Quentin`))
                (`KismetSystemLibrary.MoveComponentTo` _door _relativelocation (struct :`Yaw` -100.0) false false (`self.Over Time`) true :!label _label_2)
                (else
                  (`KismetSystemLibrary.MoveComponentTo` _door _relativelocation (struct :`Yaw` 100.0) false false (`self.Over Time`) true :!label _label_3))))))))))

(fn `UserConstructionScript`
  (`parent.UserConstructionScript`))