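; Placement marker for a neighbor AI item drop location, shown as either a box or a chair.
; The construction script sets the preview static mesh from the State value.
; The RunBeginFunction event destroys that mesh component, and the file holds no drop logic of its own.
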(event `self.Run Begin Function`
  (`ActorComponent.K2_DestroyComponent` (`self.StaticMesh`)))

(fn `UserConstructionScript`
  (`parent.UserConstructionScript`)
  (switch `/Game/Main/Characters/AI/Blueprints/Neighbor/E_Item_State` (`self.State`)
    (:`NewEnumerator0`
      (`StaticMeshComponent.SetStaticMesh` (`self.StaticMesh`) "/Game/Main/Objects/Alpha/Meshes/SM_SM_Box_00_mo.SM_SM_Box_00_mo"))
    (:`NewEnumerator1`
      (`StaticMeshComponent.SetStaticMesh` (`self.StaticMesh`) "/Game/Main/Objects/Items/O_SM_Chair_01_LOD0_mo.O_SM_Chair_01_LOD0_mo"))))