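; Base Neighbor AI character that idles, hunts and chases the player (Quentin).
; SetState switches behavior tree, walk speed and music per state, while blackboard tasks select actions, randomly when idle.
; Sightings inside its tagged AttackZone trigger Chase, perceived objects trigger Hunt, and touching Quentin mid-chase pauses sensing.
; It also carries an item inventory, reacts briefly to fast item hits, and provides animation and transform-lerp helpers.
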(event `self.Box.OnComponentBeginOverlap`
  (params (OverlappedComponent :type "PrimitiveComponent Object Reference") (OtherActor :type "Actor Object Reference") (OtherComp :type "PrimitiveComponent Object Reference") (OtherBodyIndex :type Integer) (bFromSweep :type Boolean) (SweepResult :type "HitResult Structure (by ref)"))
  (bind _bp_sensing (`self.BP_Sensing`))
  (cast `/Game/Main/Characters/Quentin/Blueprint/CH_Quentin` OtherActor)
  (if (`|EnumEquality` (`self.State`) "NewEnumerator4")
    (`/Engine/EditorBlueprintResources/StandardMacros.DoOnce` false :!label _label
      (:`Completed`
        (set `/Game/Main/Characters/AI/Neighbor/BP_Sensing.Enabled?` false _bp_sensing)
        (`self.Set State` "NewEnumerator0")
        (`self.Set Task Manual` "NewEnumerator15")
        (`KismetSystemLibrary.Delay` 10.0)
        (set `/Game/Main/Characters/AI/Neighbor/BP_Sensing.Enabled?` true _bp_sensing)
        (goto _label :!via `Reset`)))))

(event `Update Neighbor Anim Task`
  (params (`Neighbor Anim Task` :type "/Game/Main/Characters/AI/Neighbor/Enums/E_Neighbor_Anim_Tasks Enum" :default "NewEnumerator0"))
  (set `self.Neighbor Anim Task` `Neighbor Anim Task`)
  (`KismetSystemLibrary.Delay` 0.8)
  (set `self.Neighbor Anim Task` "NewEnumerator0"))

(event `Constant`
  (`KismetSystemLibrary.K2_SetTimerDelegate` (delegate `Constant`) 0.05 true)
  (bind _output (`self.Get Held Item`))
  (`/Engine/EditorBlueprintResources/StandardMacros.IsValid` _output
    (:`Is Valid`
      (set `self.Holding` true)
      (set `self.Two Handed` (`/Game/Main/Objects/Blueprint/Base/BP_Base_Item.Two Handed` _output)))
    (:`Is Not Valid`
      (set `self.Holding` false))))

(event `On See`
  (params (`See Player` :type Boolean))
  (bind _state (`self.State`))
  ;[1 1 1] Toggle
  ; Chasing/Hunt/Idle
  (if `See Player`
    (if (`self.IsOverlappingActor` (`self.Attack Zone`) (`/Game/Main/Objects/HNAR_Function_Library.Find Quentin`))
      (if (`self.Can See Player`)
        (if (not (`|EnumEquality` (`self.State`) "NewEnumerator0"))
          (bind _asch_quentin (cast `/Game/Main/Characters/Quentin/Blueprint/CH_Quentin` (`GameplayStatics.GetPlayerCharacter` 0)))
          (set `self.Estimated Quentin Location` (`self.K2_GetActorLocation` _asch_quentin))
          (`|ExecutionSequence`
            (:`then_0`
              (if (not (`|EnumEquality` (`self.State`) "NewEnumerator4"))
                (`self.Set State` "NewEnumerator4")
                (`self.Set Task Manual` "NewEnumerator9"))
              (`self.Update Can See Quentin` true))
            (:`then_1`
              (`KismetSystemLibrary.RetriggerableDelay` (`self.Lose Time`))
              (`self.Update Can See Quentin` false)))))
      (elif (or (`|EnumEquality` _state "NewEnumerator4") (`|EnumEquality` _state "NewEnumerator2") (`|EnumEquality` _state "NewEnumerator3"))
        (`self.Set State` "NewEnumerator0")
        (`self.Set Task Manual` "NewEnumerator19")))))

(event `self.Mesh.OnComponentHit`
  (params (HitComponent :type "PrimitiveComponent Object Reference") (OtherActor :type "Actor Object Reference") (OtherComp :type "PrimitiveComponent Object Reference") (NormalImpulse :type "Vector Structure") (Hit :type "HitResult Structure (by ref)"))
  (bind _asbp_base_item (cast `/Game/Main/Objects/Blueprint/Base/BP_Base_Item` OtherActor))
  (`KismetSystemLibrary.PrintString` "Hello")
  (if (>= (`KismetMathLibrary.VSize` (`self.GetVelocity` _asbp_base_item)) 200.0)
    (if (not (`|EnumEquality` (`self.State`) "NewEnumerator0"))
      (`/Engine/EditorBlueprintResources/StandardMacros.DoOnce` false :!label _label_2
        (:`Completed`
          (`self.Set Speed` (`self.Idle Speed`))
          (set `self.Neighbor Anim Task` "NewEnumerator8")
          (`KismetSystemLibrary.Delay` 0.5)
          (set `self.Neighbor Anim Task` "NewEnumerator0")
          (`self.Reset Speed`)
          (goto _label_2 :!via `Reset`))))))

(event `self.ReceivePossessed`
  (params (NewController :type "Controller Object Reference"))
  (`self.Constant`)
  (`AIController.RunBehaviorTree` (`AIBlueprintHelperLibrary.GetAIController` self) "/Game/Main/Characters/AI/Neighbor/Tasks/BT_Neighbor_None.BT_Neighbor_None")
  (`self.Set State` "NewEnumerator1")
  (`|ExecutionSequence`
    (:`then_0`
      (`self.Set Task Random`)
      (bind _outactors (`GameplayStatics.GetAllActorsOfClassWithTag` "/Game/Main/Characters/AI/Blueprints/BP_AttackZone.BP_AttackZone_C" (`self.Neighbor Tag`)))
      (for _array_element _outactors
        (`KismetSystemLibrary.PrintString` "Searching for attack zone")
        (bind _output_get (set `self.Attack Zone` _array_element))
        (`/Engine/EditorBlueprintResources/StandardMacros.IsValid` _output_get
          (:`Is Valid`
            (`KismetSystemLibrary.PrintString` "Attack Zone Found" true true (struct :`R` 0.070345 :`G` 1.0 :`A` 1.0))
            (`KismetSystemLibrary.PrintString` (`KismetSystemLibrary.GetDisplayName` _output_get) true true (struct :`R` 0.070345 :`G` 1.0 :`A` 1.0)))
          (:`Is Not Valid`
            (`KismetSystemLibrary.PrintString` "Attack Zone NOT Found" true true (struct :`R` 1.0 :`G` 0.142179 :`A` 1.0))
            (`KismetSystemLibrary.PrintString` "Please Add A BP_AttackZone into the level")))))
    (:`then_1`
      (bind _outactors_2 (`GameplayStatics.GetAllActorsOfClassWithTag` "/Game/Main/Characters/AI/Blueprints/BP_Respawn_Point.BP_Respawn_Point_C" (`self.Neighbor Tag`)))
      (for _array_element_2 _outactors_2
        (set `self.Respawn Point` _array_element_2)))))

(event `self.AIPerception.OnTargetPerceptionUpdated`
  (params (Actor :type "Actor Object Reference") (Stimulus :type "AIStimulus Structure"))
  (bind _state (`self.State`))
  (bind _asbp_base_object (cast `/Game/Main/Objects/Blueprint/Base/BP_Base_Object` Actor))
  (if (not (or (`|EnumEquality` _state "NewEnumerator4") (`|EnumEquality` _state "NewEnumerator0")))
    (set `self.Estimated Quentin Location` (`SceneComponent.K2_GetComponentLocation` (`/Game/Main/Objects/Blueprint/Base/BP_Base_Object.Neighbor Location` _asbp_base_object)))
    (`self.Set Task Manual` "NewEnumerator7")
    (`KismetSystemLibrary.Delay` 0.05)
    (`self.Set Task Manual` "NewEnumerator18")
    (if (not (`|EnumEquality` (`self.State`) "NewEnumerator2"))
      (`self.Set State` "NewEnumerator2")
      (`GameplayStatics.PlaySound2D` (`self.Notif`) 1.0 1.0 0.0 null null))))

(event `Lerp Location and Rotation`
  (params (`New Location` :type "Vector Structure") (`New Rotation` :type "Rotator Structure"))
  (`self.Lerp Location` `New Location`)
  (`self.Lerp Rotation` `New Rotation`))

(event `Lerp Location`
  (params (`New Location` :type "Vector Structure"))
  (bind (_direction _alpha) (`Timeline|Move AI` :!via `PlayFromStart`)
    (:`Update`
      (`self.K2_SetActorLocation` (`KismetMathLibrary.VLerp` (`self.K2_GetActorLocation`) `New Location` _alpha)))))

(event `Lerp Rotation`
  (params (`New Rotation` :type "Rotator Structure"))
  (bind (_direction _alpha) (`Timeline|Rotate Player` :!via `PlayFromStart`)
    (:`Update`
      (`self.K2_SetActorRotation` (`KismetMathLibrary.RLerp` (`self.K2_GetActorRotation`) `New Rotation` _alpha true)))))

(fn `Drop`
  (returns (Item :type "/Game/Main/Objects/Blueprint/Base/BP_Base_Item Object Reference"))
  (bind _item (`self.Item`))
  (bind _item_2 (`self.Item`))
  (bind _item_3 (`self.Item`))
  (bind (_returnvalue_location _returnvalue_rotation) (`KismetMathLibrary.BreakTransform` (`SceneComponent.K2_GetComponentToWorld` (`self.Drop Location`))))
  (bind (_transform_origin_location _transform_origin_rotation _transform_origin_scale) (`KismetMathLibrary.BreakTransform` (`/Game/Main/Objects/Blueprint/Base/BP_Base_Object.Transform Origin` _item)))
  (`/Game/Main/Objects/Blueprint/Base/BP_Base_Item.Drop` _item_3)
  (`SceneComponent.K2_DetachFromComponent` (`Actor.RootComponent` _item_2) "KeepRelative" "KeepRelative" "KeepRelative" true)
  (`self.K2_SetActorTransform` _item (`KismetMathLibrary.MakeTransform` _returnvalue_location _returnvalue_rotation _transform_origin_scale) false false)
  (`KismetArrayLibrary.Array_RemoveItem` (`self.Inventory`) _item_3)
  (return _item_2))

(fn `Get Held Item`
  (returns (Output :type "/Game/Main/Objects/Blueprint/Base/BP_Base_Item Object Reference"))
  (return (`|GetArrayItem` (`self.Inventory`) (`self.Selected Item`))))

(fn `Get Montage Array`
  (params (`Selected Montage` :type Integer))
  (returns (Montage :type "AnimMontage Object Reference"))
  (return (`|GetArrayItem` (`self.Montage Array`) `Selected Montage`)))

(fn `Locate Items`
  (params (Name :type Name))
  (returns (`Array Element` :type "/Game/Main/Objects/Blueprint/Base/BP_Base_Object Object Reference"))
  (bind _outactors (`GameplayStatics.GetAllActorsOfClassWithTag` "/Game/Main/Objects/Blueprint/Base/BP_Base_Object.BP_Base_Object_C" Name))
  (`KismetArrayLibrary.Array_Shuffle` _outactors)
  (for _array_element _outactors
    _)
  (`/Engine/EditorBlueprintResources/StandardMacros.IsValid` _array_element
    (:`Is Valid`
      _)
    (:`Is Not Valid`
      (`self.Set Task Random`)))
  (return _array_element))

(fn `Pick Up`
  (`/Game/Main/Objects/Blueprint/Base/BP_Base_Item.Pick Up` (`self.Item`))
  (`self.K2_AttachToComponent` (`self.Item`) (`self.Items`) "None" "SnapToTarget" "SnapToTarget" "SnapToTarget" true)
  (bind _returnvalue (`KismetArrayLibrary.Array_Add` (`self.Inventory`) (`self.Item`)))
  (set `self.Selected Item` _returnvalue)
  (return))

(fn `Reset Speed`
  (switch `/Game/Main/Characters/AI/Neighbor/Enums/E_Neighbor_State` (`self.State`)
    (:`NewEnumerator0`
      (`self.Set Speed` 0.0))
    (:`NewEnumerator1`
      (`self.Set Speed` (`self.Idle Speed`)))
    (:`NewEnumerator2`
      (`self.Set Speed` (`self.Hunt Speed`)))
    (:`NewEnumerator3`
      (`self.Set Speed` (`self.Idle Speed`)))
    (:`NewEnumerator4`
      (`self.Set Speed` (`self.Chase Speed`)))))

(fn `Set Speed`
  (params (`New Speed` :type "Float (double-precision)"))
  (set `CharacterMovementComponent.MaxWalkSpeed` `New Speed` (`self.CharacterMovement`)))

(fn `Set State`
  (params (`New State` :type "/Game/Main/Characters/AI/Neighbor/Enums/E_Neighbor_State Enum" :default "NewEnumerator0"))
  (bind _charactermovement (`self.CharacterMovement`))
  (bind _returnvalue (`AIBlueprintHelperLibrary.GetAIController` self))
  (bind _output_get (set `self.State` `New State`))
  (`BlackboardComponent.SetValueAsEnum` (`AIBlueprintHelperLibrary.GetBlackboard` self) "State" _output_get)
  (switch `/Game/Main/Characters/AI/Neighbor/Enums/E_Neighbor_State` _output_get
    (:`NewEnumerator0`
      (`self.Set Speed` 0.0)
      (`AIController.RunBehaviorTree` _returnvalue "/Game/Main/Characters/AI/Neighbor/Tasks/BT_Neighbor_None.BT_Neighbor_None")
      (`AudioComponent.Stop` (`self.Hunt Music`))
      (`AudioComponent.Stop` (`self.Chase Music`))
      (`AudioComponent.Stop` (`self.Ambient Music`)))
    (:`NewEnumerator1`
      (`self.Set Speed` (`self.Idle Speed`))
      (`AIController.RunBehaviorTree` _returnvalue "/Game/Main/Characters/AI/Neighbor/Tasks/BT_Neighbor_Idle.BT_Neighbor_Idle")
      (`AudioComponent.FadeOut` (`self.Hunt Music`) 2.0 0.0 "Linear")
      (`AudioComponent.FadeOut` (`self.Chase Music`) 2.0 0.0 "Linear")
      (`self.Set Task Random`)
      (if (not (`AudioComponent.IsPlaying` (`self.Ambient Music`)))
        (`AudioComponent.Play` (`self.Ambient Music`) 0.0)))
    (:`NewEnumerator2`
      (`self.Set Speed` (`self.Hunt Speed`))
      (`AIController.RunBehaviorTree` _returnvalue "/Game/Main/Characters/AI/Neighbor/Tasks/BT_Neighbor_Hunt.BT_Neighbor_Hunt")
      (`CharacterMovementComponent.SetMovementMode` _charactermovement "MOVE_Walking" 0)
      (`AudioComponent.FadeOut` (`self.Ambient Music`) 2.0 0.0 "Linear")
      (`AudioComponent.FadeOut` (`self.Chase Music`) 2.0 0.0 "Linear")
      (if (not (`AudioComponent.IsPlaying` (`self.Hunt Music`)))
        (`AudioComponent.Play` (`self.Hunt Music`) 0.0)))
    (:`NewEnumerator3`
      (`self.Set Speed` (`self.Idle Speed`))
      (`AIController.RunBehaviorTree` _returnvalue "/Game/Main/Characters/AI/Neighbor/Tasks/BT_Neighbor_Seen.BT_Neighbor_Seen")
      (`CharacterMovementComponent.SetMovementMode` _charactermovement "MOVE_Walking" 0 :!label _label)
      (`AudioComponent.FadeOut` (`self.Hunt Music`) 2.0 0.0 "Linear")
      (`AudioComponent.FadeOut` (`self.Ambient Music`) 2.0 0.0 "Linear")
      (if (not (`AudioComponent.IsPlaying` (`self.Chase Music`)))
        (`AudioComponent.Play` (`self.Chase Music`) 0.0)))
    (:`NewEnumerator4`
      (`self.Set Speed` (`self.Chase Speed`))
      (`AIController.RunBehaviorTree` _returnvalue "/Game/Main/Characters/AI/Neighbor/Tasks/BT_Neighbor_Chase.BT_Neighbor_Chase")
      (goto _label))))

(fn `Set Task Manual`
  (params (`New Task` :type "/Game/Main/Characters/AI/Neighbor/Enums/E_Neighbor_Tasks Enum" :default "NewEnumerator0"))
  (bind _output_get (set `self.Neighbor Task` `New Task`))
  (`BlackboardComponent.SetValueAsEnum` (`AIBlueprintHelperLibrary.GetBlackboard` self) "Neighbor Task" _output_get)
  (return))

(fn `Set Task Random`
  (locals (Selection :type Integer :default 0))
  (bind _returnvalue (`AIBlueprintHelperLibrary.GetBlackboard` self))
  (bind _output_get (set `local.Selection` (`KismetMathLibrary.RandomIntegerInRange` 0 5) :!label _label))
  (if (`KismetStringLibrary.EqualEqual_StrStr` (`|GetArrayItem` (`self.IdleTasksFilter`) _output_get) "1")
    (switch `int` _output_get
      (:`0`
        (bind _output_get_2 (set `self.Neighbor Task` "NewEnumerator12"))
        (`BlackboardComponent.SetValueAsEnum` _returnvalue "Neighbor Task" _output_get_2))
      (:`1`
        (bind _output_get_3 (set `self.Neighbor Task` "NewEnumerator8"))
        (`BlackboardComponent.SetValueAsEnum` _returnvalue "Neighbor Task" _output_get_3))
      (:`2`
        (bind _output_get_4 (set `self.Neighbor Task` "NewEnumerator13"))
        (`BlackboardComponent.SetValueAsEnum` _returnvalue "Neighbor Task" _output_get_4))
      (:`3`
        (bind _output_get_5 (set `self.Neighbor Task` "NewEnumerator2"))
        (`BlackboardComponent.SetValueAsEnum` _returnvalue "Neighbor Task" _output_get_5))
      (:`4`
        (bind _output_get_6 (set `self.Neighbor Task` "NewEnumerator4"))
        (`BlackboardComponent.SetValueAsEnum` _returnvalue "Neighbor Task" _output_get_6))
      (:`5`
        (bind _output_get_7 (set `self.Neighbor Task` "NewEnumerator3"))
        (`BlackboardComponent.SetValueAsEnum` _returnvalue "Neighbor Task" _output_get_7)))
    (return)
    (else
      (goto _label))))

(fn `Update Can See Quentin`
  (params (`Can See Quentin` :type Boolean))
  (bind _output_get (set `self.Can See Quentin` `Can See Quentin`))
  (`BlackboardComponent.SetValueAsBool` (`AIBlueprintHelperLibrary.GetBlackboard` self) "Can See Quentin" _output_get))

(fn `Update Mood`
  (params (NewMood :type "/Game/Main/Characters/AI/Neighbor/Enums/E_Neighbor_Mood Enum" :default "NewEnumerator0")))

(fn `UserConstructionScript`
  (`parent.UserConstructionScript`)
  (`SkinnedMeshComponent.SetLeaderPoseComponent` (`self.Head`) (`self.Mesh`) false))