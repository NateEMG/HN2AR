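; BP_Sensing is a sight component for AI characters that detects the player.
; On BeginPlay it targets player 0 and starts a looping timer that runs the sight check.
; The check requires an unblocked Visibility trace to the player, within SensingRange and ConeAngle of the forward vector.
; Each result, seen or not, goes to the owning BP_Base_AI's OnSee, with optional cone drawing and failure messages for debugging.
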(event `self.ReceiveBeginPlay`
  (set `self.Target` (`GameplayStatics.GetPlayerCharacter` 0))
  (`self.Begin Sensing`))

(event `Begin Sensing`
  (bind _returnvalue (`KismetSystemLibrary.K2_SetTimerDelegate` (delegate `Sense`) (`self.Sensing Interval`) true))
  (set `self.Sensing Timer Ref` _returnvalue))

(event `Sense`
  (bind _see_target (`self.Sense For Target`))
  (bind _asbp_base_ai (cast `/Game/Main/Characters/AI/Neighbor/BP_Base_AI` (`self.GetOwner`)))
  (`/Engine/EditorBlueprintResources/StandardMacros.IsValid` _asbp_base_ai
    (:`Is Valid`
      (`/Game/Main/Characters/AI/Neighbor/BP_Base_AI.On See` _asbp_base_ai _see_target))))

(fn `Debug Message`
  (params (InString :type String))
  (if (`self.Debug`)
    (`KismetSystemLibrary.PrintString` InString)))

(fn `Sense For Target`
  (returns (`See Target` :type Boolean))
  (locals (`Current Hit Result` :type "HitResult Structure") (`Can See` :type Boolean))
  (bind _returnvalue_location (`KismetMathLibrary.BreakTransform` (`self.K2_GetComponentToWorld`)))
  (bind (_current_hit_result_bblockinghit _current_hit_result_binitialoverlap _current_hit_result_time _current_hit_result_distance) (`GameplayStatics.BreakHitResult` (`local.Current Hit Result`)))
  (bind (_current_hit_result_bblockinghit_2 _current_hit_result_binitialoverlap_2 _current_hit_result_time_2 _current_hit_result_distance_2 _current_hit_result_location _current_hit_result_impactpoint _current_hit_result_normal _current_hit_result_impactnormal _current_hit_result_physmat _current_hit_result_hitactor) (`GameplayStatics.BreakHitResult` (`local.Current Hit Result`)))
  (bind _cone_angle (`self.Cone Angle`))
  (bind _returnvalue (`KismetMathLibrary.DegAcos` (`KismetMathLibrary.Dot_VectorVector` (`self.GetForwardVector`) (`KismetMathLibrary.GetDirectionUnitVector` (`self.K2_GetComponentLocation`) (`Actor.K2_GetActorLocation` (`self.Target`))))))
  (set `local.Can See` false)
  (if (`self.Debug`)
    (`KismetSystemLibrary.DrawDebugConeInDegrees` _returnvalue_location (`self.GetForwardVector`) (`self.Sensing Range`) _cone_angle _cone_angle 12 (struct :`R` 1.0 :`G` 1.0 :`B` 1.0 :`A` 1.0) (`self.Sensing Interval`) 1.0))
  (bind (_outhit _returnvalue_2) (`KismetSystemLibrary.LineTraceSingle` (`self.K2_GetComponentLocation`) (`Actor.K2_GetActorLocation` (`self.Target`)) "TraceTypeQuery1" false (`|MakeArray` (`self.GetOwner`)) (`self.Trace Debug`)))
  (if _returnvalue_2
    (set `local.Current Hit Result` _outhit)
    (if (== _current_hit_result_hitactor (`self.Target`))
      (if (<= _current_hit_result_distance (`self.Sensing Range`))
        (if (<= _returnvalue (`self.Cone Angle`))
          (bind _output_get (set `local.Can See` true))
          (return _output_get)
          (else
            (`self.Debug Message` (`KismetStringLibrary.Concat_StrStr` "Target is out of peripheral vision" "Angle =" (`KismetStringLibrary.Conv_DoubleToString` _returnvalue)))
            (bind _output_get_2 (set `local.Can See` false))
            (return _output_get_2)))
        (else
          (`self.Debug Message` "Target is out of range")))
      (else
        (`self.Debug Message` "Sensing is blocked by wall or object")))
    (bind _output_get_3 (set `local.Can See` false))
    (return _output_get_3)
    (else
      (`self.Debug Message` "Couldn't see target")
      (bind _output_get_4 (set `local.Can See` false))
      (return _output_get_4))))