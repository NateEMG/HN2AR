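; Base AI character for the Neighbor, driven by a state machine that switches between None, Idle, Hunt, Seen and Chase.
; UpdateState writes the state to the Blackboard, sets walk speed, runs that state's behavior tree and fades between ambient, hunt and chase music with stingers.
; Possession starts Idle, and sighting CH_Quentin through PawnSensing triggers Chase.
; Tick prints the current state for debugging.
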(event `self.ReceiveTick`
  (params (DeltaSeconds :type "Float (single-precision)"))
  (`KismetSystemLibrary.PrintString` (`|GetEnumeratorNameAsString` (`self.State`)) true true (struct :`G` 0.66 :`B` 1.0 :`A` 1.0) 0.0001))

(event `self.PawnSensing.OnSeePawn`
  (params (Pawn :type "Pawn Object Reference"))
  (cast `/Game/Main/Characters/Quentin/Blueprint/CH_Quentin` Pawn)
  (if (not (`|EnumEquality` (`self.State`) "NewEnumerator4"))
    (`self.Update State` "NewEnumerator4")))

(event `self.ReceivePossessed`
  (params (NewController :type "Controller Object Reference"))
  (`AIController.RunBehaviorTree` (`AIBlueprintHelperLibrary.GetAIController` self) "/Game/Main/Characters/AI/BT_Neighbor_None.BT_Neighbor_None")
  (`self.Update State` "NewEnumerator1"))

(fn `Set Speed`
  (params (`New Speed` :type "Float (double-precision)"))
  (set `CharacterMovementComponent.MaxWalkSpeed` `New Speed` (`self.CharacterMovement`)))

(fn `Update State`
  (params (`New State` :type "/Game/Main/Characters/AI/E_Neighbor_State Enum" :default "NewEnumerator0"))
  (bind _returnvalue (`AIBlueprintHelperLibrary.GetAIController` self))
  (bind _output_get (set `self.State` `New State`))
  (`BlackboardComponent.SetValueAsEnum` (`AIBlueprintHelperLibrary.GetBlackboard` self) "State" _output_get)
  (switch `/Game/Main/Characters/AI/E_Neighbor_State` _output_get
    (:`NewEnumerator0`
      (`self.Set Speed` 0.0)
      (`AIController.RunBehaviorTree` _returnvalue "/Game/Main/Characters/AI/BT_Neighbor_None.BT_Neighbor_None")
      (`AudioComponent.Stop` (`self.Hunt Music`))
      (`AudioComponent.Stop` (`self.Chase Music`))
      (`AudioComponent.Stop` (`self.Ambient Music`)))
    (:`NewEnumerator1`
      (`self.Set Speed` (`self.Idle Speed`))
      (`AIController.RunBehaviorTree` _returnvalue "/Game/Main/Characters/AI/BT_Neighbor_Idle.BT_Neighbor_Idle")
      (`AudioComponent.FadeOut` (`self.Hunt Music`) 2.0 0.0 "Linear")
      (`AudioComponent.FadeOut` (`self.Chase Music`) 2.0 0.0 "Linear")
      (if (not (`AudioComponent.IsPlaying` (`self.Ambient Music`)))
        (`AudioComponent.Play` (`self.Ambient Music`) 0.0)))
    (:`NewEnumerator2`
      (`self.Set Speed` (`self.Hunt Speed`))
      (`AIController.RunBehaviorTree` _returnvalue "/Game/Main/Characters/AI/BT_Neighbor_Hunt.BT_Neighbor_Hunt")
      (`AudioComponent.FadeOut` (`self.Ambient Music`) 2.0 0.0 "Linear")
      (`AudioComponent.FadeOut` (`self.Chase Music`) 2.0 0.0 "Linear")
      (if (not (`AudioComponent.IsPlaying` (`self.Hunt Music`)))
        (`AudioComponent.Play` (`self.Hunt Music`) 0.0)
        (`GameplayStatics.PlaySound2D` "/Game/Main/Sounds/Music/Hideout_event_2.Hideout_event_2" 1.0 1.0 0.0 null null)))
    (:`NewEnumerator3`
      (`self.Set Speed` (`self.Idle Speed`))
      (`AIController.RunBehaviorTree` _returnvalue "/Game/Main/Characters/AI/BT_Neighbor_Seen.BT_Neighbor_Seen")
      (`AudioComponent.FadeOut` (`self.Hunt Music`) 2.0 0.0 "Linear" :!label _label)
      (`AudioComponent.FadeOut` (`self.Ambient Music`) 2.0 0.0 "Linear")
      (if (not (`AudioComponent.IsPlaying` (`self.Chase Music`)))
        (`AudioComponent.Play` (`self.Chase Music`) 0.0)
        (`GameplayStatics.PlaySound2D` "/Game/Main/Sounds/Music/Hideout_event_1.Hideout_event_1" 1.0 1.0 0.0 null null)))
    (:`NewEnumerator4`
      (`self.Set Speed` (`self.Chase Speed`))
      (`AIController.RunBehaviorTree` _returnvalue "/Game/Main/Characters/AI/BT_Neighbor_Chase.BT_Neighbor_Chase")
      (goto _label))))

(fn `UserConstructionScript`)