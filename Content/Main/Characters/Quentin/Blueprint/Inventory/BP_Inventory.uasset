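; BP_Inventory is an actor that visually displays the items the player character Quentin carries in his inventory.
; When its Opened event runs, it casts the player character to CH_Quentin and stores the reference.
; It then checks the first five inventory slots and, for each valid item, copies that item's static mesh onto the matching display mesh component.
; Empty slots are left untouched rather than cleared.
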(event `Opened`
  (bind _asch_quentin (cast `/Game/Main/Characters/Quentin/Blueprint/CH_Quentin` (`GameplayStatics.GetPlayerCharacter` 0)))
  (bind _output_get (set `self.Quentin` _asch_quentin))
  (bind _inventory (`/Game/Main/Characters/Quentin/Blueprint/CH_Quentin.Inventory` _output_get))
  (bind _output (`|GetArrayItem` _inventory))
  (`/Engine/EditorBlueprintResources/StandardMacros.IsValid` _output
    (:`Is Valid`
      (`StaticMeshComponent.SetStaticMesh` (`self.Item_1`) (`StaticMeshComponent.StaticMesh` (`/Game/Main/Objects/Blueprint/Base/BP_Base_Item.Mesh` _output))))
    (:`Is Not Valid`
      _))
  (bind _output_2 (`|GetArrayItem` _inventory 1))
  (`/Engine/EditorBlueprintResources/StandardMacros.IsValid` _output_2
    (:`Is Valid`
      (`StaticMeshComponent.SetStaticMesh` (`self.Item_2`) (`StaticMeshComponent.StaticMesh` (`/Game/Main/Objects/Blueprint/Base/BP_Base_Item.Mesh` _output_2))))
    (:`Is Not Valid`
      _))
  (bind _output_3 (`|GetArrayItem` _inventory 2))
  (`/Engine/EditorBlueprintResources/StandardMacros.IsValid` _output_3
    (:`Is Valid`
      (`StaticMeshComponent.SetStaticMesh` (`self.Item_3`) (`StaticMeshComponent.StaticMesh` (`/Game/Main/Objects/Blueprint/Base/BP_Base_Item.Mesh` _output_3))))
    (:`Is Not Valid`
      _))
  (bind _output_4 (`|GetArrayItem` _inventory 3))
  (`/Engine/EditorBlueprintResources/StandardMacros.IsValid` _output_4
    (:`Is Valid`
      (`StaticMeshComponent.SetStaticMesh` (`self.Item_4`) (`StaticMeshComponent.StaticMesh` (`/Game/Main/Objects/Blueprint/Base/BP_Base_Item.Mesh` _output_4))))
    (:`Is Not Valid`
      _))
  (bind _output_5 (`|GetArrayItem` _inventory 4))
  (`/Engine/EditorBlueprintResources/StandardMacros.IsValid` _output_5
    (:`Is Valid`
      (`StaticMeshComponent.SetStaticMesh` (`self.Item_5`) (`StaticMeshComponent.StaticMesh` (`/Game/Main/Objects/Blueprint/Base/BP_Base_Item.Mesh` _output_5))))))

(fn `UserConstructionScript`)